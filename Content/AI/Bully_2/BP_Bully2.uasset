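; BP_Bully2 is an AI bully that detects the player through AI Perception and feeds its controller's Blackboard.
; Sensing the player sets TargetActor and TargetLocation; a failed stimulus copies TargetLocation to InvestigateLocation and clears TargetActor.
; A looping timer extrapolates a fixed distance along the target's last movement direction and writes PredictedLocation.
; The controller reference is only cached on perception updates.
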(event `PredictPlayerMovement`
  (bind _returnvalue (`BlackboardComponent.GetValueAsObject` (`AIController.Blackboard` (`self.Bully Controller Ref`)) "TargetActor"))
  (`/Engine/EditorBlueprintResources/StandardMacros.IsValid` _returnvalue
    (:`Is Valid`
      (bind _assp_player_character (cast `/Game/Player/SP_PlayerCharacter` _returnvalue))
      (bind _output_get (set `self.CurrentLocation` (`self.K2_GetActorLocation` _assp_player_character)))
      (bind _output_get_2 (set `self.Direction` (`KismetMathLibrary.Normal` (- _output_get (`self.LastPlayerPosition`)))))
      (bind _output_get_3 (set `self.PredictedLocation` (+ (`self.CurrentLocation`) (* _output_get_2 500.0))))
      (`BlackboardComponent.SetValueAsVector` (`AIController.Blackboard` (`self.Bully Controller Ref`)) "PredictedLocation" _output_get_3)
      (set `self.LastPlayerPosition` (`self.CurrentLocation`)))))

(event `self.ReceiveBeginPlay`
  (`KismetSystemLibrary.K2_SetTimer` null "PredictPlayerMovement" (`self.PredictionUpdateRate`) true))

(event `self.AIPerception.OnTargetPerceptionUpdated`
  (params (Actor :type "Actor Object Reference") (Stimulus :type "AIStimulus Structure"))
  (bind _blackboard (`AIController.Blackboard` (`self.Bully Controller Ref`)))
  (bind _returnvalue (`BlackboardComponent.GetValueAsVector` _blackboard "TargetLocation"))
  (bind _asbp_bully_2controller (cast `/Game/AI/Bully_2/BP_Bully2Controller` (`self.GetController`)))
  (set `self.Bully Controller Ref` _asbp_bully_2controller)
  (if Stimulus_bSuccessfullySensed
    (bind _assp_player_character (cast `/Game/Player/SP_PlayerCharacter` Actor))
    (`BlackboardComponent.SetValueAsObject` _blackboard "TargetActor" _assp_player_character)
    (`BlackboardComponent.SetValueAsVector` _blackboard "TargetLocation" (`self.K2_GetActorLocation` _assp_player_character))
    (`KismetSystemLibrary.PrintString` "SEE PLAYER")
    (else
      (`KismetSystemLibrary.PrintString` "LOST PLAYER")
      (`BlackboardComponent.SetValueAsVector` _blackboard "InvestigateLocation" _returnvalue)
      (`KismetSystemLibrary.PrintString` (`KismetStringLibrary.Concat_StrStr` "InvestigateLocation set to" (`KismetStringLibrary.Conv_VectorToString` _returnvalue)))
      (`BlackboardComponent.ClearValue` _blackboard "TargetActor"))))

(fn `UserConstructionScript`)