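; Quest manager actor that holds the player's quest list and marks quests as completed.
; On BeginPlay it binds to OnQuestCompleted, whose handler sets the matching QuestID's entry to completed, then prints all quest IDs for debugging.
; A separate load function, not called within this Blueprint, copies QuestsData from the SP_GameInstance save data.
; Completion updates only the local array, with no write-back to the save data here.
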(event `self.ReceiveBeginPlay`
  (add `self.OnQuestCompleted` (delegate `evCompleteQuest`)))

(event `evCompleteQuest` :!signature `self.OnQuestCompleted`
  (params (QuestToComplete :type Name))
  (`|ExecutionSequence`
    (:`then_0`
      (`self.fnCompleteQuest` QuestToComplete))
    (:`then_1`
      (for _array_element (`self.Quests`)
        (`KismetSystemLibrary.PrintString` (`KismetStringLibrary.Conv_NameToString` (`.QuestID_2_AB1D96064D99289137A095AA09FE9A4F` (break `/Game/Blueprints/Structs/STR_MainQuests` _array_element))))))))

(fn `fnCompleteQuest`
  (params (QuestToComplete :type Name))
  (returns (Success :type Boolean))
  (bind _questtocomplete (`local.QuestToComplete`))
  (for (_array_element _array_index) (`self.Quests`)
    (if (== (`.QuestID_2_AB1D96064D99289137A095AA09FE9A4F` (break `/Game/Blueprints/Structs/STR_MainQuests` _array_element)) QuestToComplete)
      (`KismetArrayLibrary.Array_Set` (`self.Quests`) _array_index (make `/Game/Blueprints/Structs/STR_MainQuests` _questtocomplete true))
      (`KismetSystemLibrary.PrintString` (`KismetStringLibrary.Concat_StrStr` (`KismetStringLibrary.Conv_NameToString` _questtocomplete) " is completed."))
      (return true))))

(fn `fnLoadCurrentQuests`
  (bind _assp_game_instance (cast `/Game/SP_GameInstance` (`GameplayStatics.GetGameInstance`)))
  (bind _questsdata (`/Game/SaveData/SaveData_PlayerData.QuestsData` (`/Game/SP_GameInstance.SavePlayerData` _assp_game_instance)))
  (for _array_element _questsdata
    (`KismetSystemLibrary.PrintString` "Hello" true true (struct :`G` 0.66 :`B` 1.0 :`A` 1.0) 2.0 (`.QuestID_2_AB1D96064D99289137A095AA09FE9A4F` (break `/Game/Blueprints/Structs/STR_MainQuests` _array_element))))
  (set `self.Quests` _questsdata))

(fn `UserConstructionScript`)