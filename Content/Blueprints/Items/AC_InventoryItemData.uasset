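; Item data component that lets its owning world actor be picked up into the player's inventory or examined up close.
; Interact passes the item ID and quantity to the player's inventory component and destroys the owner on success.
; Examine shifts input from player to item, moves it before the camera and plays a sound, with left-mouse drag rotating it.
; The interactable, examinable and look-at queries return only false or empty values.
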(event `/Game/Blueprints/BPInterfaces/BPi_Interact.Interact`
  (params (PlayerCharacter :type "/Game/Characters/Player/SP_PlayerCharacter Object Reference"))
  (bind (_itemid_datatable _itemid_rowname) (break `DataTableRowHandle` (`self.ItemID`)))
  (bind _ac_inventory (`/Game/Characters/Player/SP_PlayerCharacter.AC_Inventory` PlayerCharacter))
  ;[1 1 1] Pick Up
  (`/Engine/EditorBlueprintResources/StandardMacros.IsValid` _ac_inventory
    (:`Is Valid`
      (bind _success (`/Game/Blueprints/Interaction/AC_Inventory.fnAddToInventory` _ac_inventory _itemid_rowname (`self.Quantity`)))
      (if _success
        (`Actor.K2_DestroyActor` (`self.GetOwner`))))))

(event `self.Examine`
  (bind _returnvalue (`GameplayStatics.GetPlayerCameraManager` 0))
  (bind _returnvalue_2 (`self.GetOwner`))
  (bind _returnvalue_3 (`GameplayStatics.GetPlayerController` 0))
  ;[1 1 1] Examine
  (`Actor.DisableInput` (`GameplayStatics.GetPlayerCharacter` 0) _returnvalue_3)
  (`Actor.EnableInput` _returnvalue_2 _returnvalue_3)
  (`Actor.K2_SetActorLocation` _returnvalue_2 (+ (`PlayerCameraManager.GetCameraLocation` _returnvalue) (* (`KismetMathLibrary.GetForwardVector` (`PlayerCameraManager.GetCameraRotation` _returnvalue)) (`self.Examine Distance`))) false false)
  (`GameplayStatics.PlaySound2D` "/Game/Audio/393824__sirbedlam__violin-scare.393824__sirbedlam__violin-scare" 0.5 1.0 0.0 null null false))

(event `InputAxisKey|MouseX`
  (params (AxisValue :type "Float (single-precision)"))
  (bind _returnvalue (`self.GetOwner`))
  ;[1 1 1] Examine
  (if (`self.IsExamining`)
    (`Actor.K2_SetActorRotation` _returnvalue (`KismetMathLibrary.ComposeRotators` (`Actor.K2_GetActorRotation` _returnvalue) (`KismetMathLibrary.MakeRotator` 0.0 0.0 (* AxisValue -5.0))) false)))

(event `Key|LeftMouseButton`
  (params (Key :type "Key Structure"))
  ;[1 1 1] Examine
  (:`Pressed`
    (set `self.IsExamining` true))
  (:`Released`
    (set `self.IsExamining` false)))

(event `InputAxisKey|MouseY`
  (params (AxisValue :type "Float (single-precision)"))
  (bind _returnvalue (`self.GetOwner`))
  ;[1 1 1] Examine
  (if (`self.IsExamining`)
    (`Actor.K2_SetActorRotation` _returnvalue (`KismetMathLibrary.ComposeRotators` (`Actor.K2_GetActorRotation` _returnvalue) (`KismetMathLibrary.MakeRotator` 0.0 (* AxisValue -5.0))) false)))

(fn `IsExaminable`
  (returns (IsExaminable :type Boolean))
  (return false))

(fn `IsInteractable`
  (returns (IsInteractable :type Boolean))
  (return false))

(fn `LookAt`
  (returns (Messege :type Text))
  (return ""))