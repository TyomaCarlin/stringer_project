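; Quest item actor that the player can pick up or examine up close.
; Interact adds its item ID and quantity to the character's inventory component and destroys the actor on success.
; Examine moves input from the character to the actor, places it in front of the camera and plays a violin scare sound, with no exit or reset logic.
; While examining, holding left mouse and moving the mouse rotates it.
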(event `/Game/Blueprints/Interaction/BPi_Interact.Interact`
  (params (PlayerCharacter :type "/Game/SP_PlayerCharacter Object Reference"))
  (bind _ac_inventory (`/Game/SP_PlayerCharacter.AC_Inventory` PlayerCharacter))
  (bind (_itemid_datatable _itemid_rowname) (break `DataTableRowHandle` (`self.ItemID`)))
  ;[1 1 1] Pick Up
  (`/Engine/EditorBlueprintResources/StandardMacros.IsValid` _ac_inventory
    (:`Is Valid`
      (bind _success (`/Game/Blueprints/Interaction/AC_Inventory.fnAddToInventory` _ac_inventory _itemid_rowname (`self.Quantity`)))
      (if _success
        (`self.K2_DestroyActor`)))))

(event `/Game/Blueprints/Interaction/BPi_Interact.Examine`
  (bind _returnvalue (`GameplayStatics.GetPlayerCameraManager` 0))
  (bind _returnvalue_2 (`GameplayStatics.GetPlayerController` 0))
  ;[1 1 1] Examine
  (`self.DisableInput` (`GameplayStatics.GetPlayerCharacter` 0) _returnvalue_2)
  (`self.EnableInput` _returnvalue_2)
  (`self.K2_SetActorLocation` (+ (`PlayerCameraManager.GetCameraLocation` _returnvalue) (* (`KismetMathLibrary.GetForwardVector` (`PlayerCameraManager.GetCameraRotation` _returnvalue)) (`self.ExamineDistance`))))
  (`GameplayStatics.PlaySound2D` "/Game/Audio/393824__sirbedlam__violin-scare.393824__sirbedlam__violin-scare" 0.5 1.0 0.0 null null false))

(event `InputAxisKey|MouseX`
  (params (AxisValue :type "Float (single-precision)"))
  ;[1 1 1] Examine
  (if (`self.IsExamining`)
    (`self.K2_SetActorRotation` (`KismetMathLibrary.ComposeRotators` (`self.K2_GetActorRotation`) (`KismetMathLibrary.MakeRotator` 0.0 0.0 (* AxisValue -5.0))))))

(event `Key|LeftMouseButton`
  (params (Key :type "Key Structure"))
  ;[1 1 1] Examine
  (:`Pressed`
    (set `self.IsExamining` true))
  (:`Released`
    (set `self.IsExamining` false)))

(event `InputAxisKey|MouseY`
  (params (AxisValue :type "Float (single-precision)"))
  ;[1 1 1] Examine
  (if (`self.IsExamining`)
    (`self.K2_SetActorRotation` (`KismetMathLibrary.ComposeRotators` (`self.K2_GetActorRotation`) (`KismetMathLibrary.MakeRotator` 0.0 (* AxisValue -5.0))))))

(fn `IsExaminable`
  (returns (IsExaminable :type Boolean))
  (return true))

(fn `IsInteractable`
  (returns (IsInteractable :type Boolean))
  (return true))

(fn `LookAt`
  (returns (Messege :type Text))
  (return ""))

(fn `UserConstructionScript`)