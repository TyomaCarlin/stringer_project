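; BP_StaticInterObject is a static interactable prop whose mesh and text are data-driven.
; The construction script looks up its row in the DT_InterProps data table and applies the mesh, description and name.
; Interact prints the description as text for a few seconds, while LookAt returns an empty value.
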(event `/Game/Blueprints/Interaction/BPi_Interact.Interact`
  (`KismetSystemLibrary.PrintText` (`self.Description`) true true (struct :`G` 0.66 :`B` 1.0 :`A` 1.0) 5.0))

(fn `LookAt`
  (returns (Messege :type Text))
  (return ""))

(fn `UserConstructionScript`
  (bind (_dt_interobjects_datatable _dt_interobjects_rowname) (break `DataTableRowHandle` (`self.DT_InterObjects`)))
  (bind _returnvalue (`|GetDataTableRow` "/Game/Blueprints/Interaction/DT_InterProps.DT_InterProps" _dt_interobjects_rowname)
    (:`then`
      (`|ExecutionSequence`
        (:`then_0`
          (`StaticMeshComponent.SetStaticMesh` (`self.StaticMesh`) (`.Mesh_10_30B2122648E0BF9C4661F7B6575DE699` (break `/Game/Blueprints/Interaction/STR_InterProps` _returnvalue))))
        (:`then_1`
          (set `self.Description` (`.Description_7_7FFFDC914BC9FF8CC7E642B663CEE76E` (break `/Game/Blueprints/Interaction/STR_InterProps` _returnvalue))))
        (:`then_2`
          (set `self.Name` (break `/Game/Blueprints/Interaction/STR_InterProps` _returnvalue)))))))