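; BP_Frame is an actor whose pivot turns in yaw when one of its four child BP_Button actors is interacted with.
; BeginPlay binds every button to one event, which picks a clockwise or counterclockwise timeline from the loop element's Clockwise flag, not the sender's.
; The timeline offsets the starting yaw, while Recharging blocks presses until it finishes.
; FnRotate, an instant 90-degree alternative, is not called here.
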(event `self.ReceiveBeginPlay`
  (for _array_element (`|MakeArray` (cast `/Game/Blueprints/Actors/BP_Button` (`ChildActorComponent.ChildActor` (`self.Button1`)) :!pure true) (cast `/Game/Blueprints/Actors/BP_Button` (`ChildActorComponent.ChildActor` (`self.Button2`)) :!pure true) (cast `/Game/Blueprints/Actors/BP_Button` (`ChildActorComponent.ChildActor` (`self.Button6`)) :!pure true) (cast `/Game/Blueprints/Actors/BP_Button` (`ChildActorComponent.ChildActor` (`self.Button5`)) :!pure true))
    (add `/Game/Blueprints/Actors/BP_Button.Interacted` _array_element (delegate `evPushed`))))

(event `evPushed`
  (bind _framepivot (`self.FramePivot`))
  (bind _start_rotation (`self.Start Rotation`))
  (bind (_relativerotation_roll _relativerotation_pitch _relativerotation_yaw) (`KismetMathLibrary.BreakRotator` (`SceneComponent.RelativeRotation` (`self.FramePivot`))))
  (bind (_relativerotation_roll_2 _relativerotation_pitch_2) (`KismetMathLibrary.BreakRotator` (`SceneComponent.RelativeRotation` _framepivot)))
  (if (not (`self.Recharging`))
    (set `self.Start Rotation` _relativerotation_yaw)
    (if (`/Game/Blueprints/Actors/BP_Button.Clockwise` (stale `self.ReceiveBeginPlay` _array_element))
      (bind (_direction _alpha) (`Timeline|Clockwise Rotation`)
        (:`Update`
          (`SceneComponent.K2_SetRelativeRotation` _framepivot (`KismetMathLibrary.MakeRotator` _relativerotation_roll_2 _relativerotation_pitch_2 (+ _start_rotation _alpha)) false false)
          (set `self.Recharging` true))
        (:`Finished`
          (set `self.Recharging` false)))
      (else
        (bind (_direction_2 _alpha_2) (`Timeline|Non-Clockwise Rotation`)
          (:`Update`
            (`SceneComponent.K2_SetRelativeRotation` _framepivot (`KismetMathLibrary.MakeRotator` _relativerotation_roll_2 _relativerotation_pitch_2 (+ _start_rotation _alpha_2)) false false)
            (set `self.Recharging` true))
          (:`Finished`
            (set `self.Recharging` false)))))))

(fn `fnRotate`
  (params (`Button Pushed` :type "/Game/Blueprints/Actors/BP_Button Object Reference") (`Start Rotation` :type "Float (double-precision)") (`Target Rotation` :type "Float (double-precision)"))
  (bind _framepivot (`self.FramePivot`))
  (bind _framepivot_2 (`self.FramePivot`))
  (bind (_relativerotation_roll _relativerotation_pitch _relativerotation_yaw) (`KismetMathLibrary.BreakRotator` (`SceneComponent.RelativeRotation` _framepivot)))
  (bind (_relativerotation_roll_2 _relativerotation_pitch_2 _relativerotation_yaw_2) (`KismetMathLibrary.BreakRotator` (`SceneComponent.RelativeRotation` _framepivot)))
  (if (`/Game/Blueprints/Actors/BP_Button.Clockwise` `Button Pushed`)
    (`SceneComponent.K2_SetRelativeRotation` _framepivot_2 (`KismetMathLibrary.MakeRotator` _relativerotation_roll_2 _relativerotation_pitch_2 (+ 90.0 _relativerotation_yaw_2)) false false)
    (set `self.Recharging` true)
    (else
      (`SceneComponent.K2_SetRelativeRotation` _framepivot_2 (`KismetMathLibrary.MakeRotator` _relativerotation_roll _relativerotation_pitch (+ -90.0 _relativerotation_yaw)) false false)
      (set `self.Recharging` true))))

(fn `UserConstructionScript`)