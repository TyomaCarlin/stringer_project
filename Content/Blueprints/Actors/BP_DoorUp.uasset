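; Interactable door actor that slides its Door component vertically to open and close, with an optional key requirement.
; Interact passes through a DoOnce, then either prints a key prompt or toggles IsClosed and plays or reverses the OpenDoor timeline.
; The timeline drives the door's relative Z and resets the DoOnce when finished.
; The key-prompt branch never resets the DoOnce, so it fires only once.
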(event `/Game/Blueprints/BPInterfaces/BPi_Interact.Interact`
  (params (PlayerCharacter :type "/Game/Player/SP_PlayerCharacter Object Reference"))
  (bind _door (`self.Door`))
  (bind (_relativelocation_x _relativelocation_y) (`KismetMathLibrary.BreakVector` (`SceneComponent.RelativeLocation` _door)))
  (`/Engine/EditorBlueprintResources/StandardMacros.DoOnce` false :!label _label
    (:`Completed`
      (if (`self.KeyRequired?`)
        (`KismetSystemLibrary.PrintString` "Get the Key")
        (elif (`self.IsClosed`)
          (set `self.IsClosed` false)
          (bind (_direction _alpha) (`Timeline|Open Door` :!label _label_2)
            (:`Update`
              (`SceneComponent.K2_SetRelativeLocation` _door (`KismetMathLibrary.MakeVector` _relativelocation_x _relativelocation_y _alpha) false false))
            (:`Finished`
              (goto _label :!via `Reset`)))
          (else
            (set `self.IsClosed` true)
            (goto _label_2 :!via `Reverse`)))))))

(fn `IsExaminable`
  (returns (IsExaminable :type Boolean))
  (return false))

(fn `IsInteractable`
  (returns (IsInteractable :type Boolean))
  (return true))

(fn `UserConstructionScript`
  (`parent.UserConstructionScript`))