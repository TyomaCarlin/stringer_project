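; Interactable door actor that either shows a locked-door description or swings open once on a timeline.
; Construction reads description and locked state from a data table row and configures hint spheres and icons.
; When locked, it pauses the game, shows a description widget and takes input until IA_Interact dismisses it and calls EvShowInventory on the player controller.
; Overlap and HUD events toggle interaction icons, with an outer icon for main goals.
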(event `self.ReceiveTick`
  (params (DeltaSeconds :type "Float (single-precision)"))
  (set `self.KeyRequired?` (`self.KeyRequired?`)))

(event `/Game/Blueprints/BPInterfaces/BPi_Interact.Interact`
  (params (PlayerCharacter :type "/Game/Player/SP_PlayerCharacter Object Reference"))
  (if (`self.KeyRequired?`)
    (`self.fnShowDescription`)
    (elif (`self.IsClosed`)
      (set `self.IsClosed` false)
      (bind (_direction _alpha) (`Timeline|Open Door`)
        (:`Update`
          (`SceneComponent.K2_SetRelativeRotation` (`self.Pivot`) (`KismetMathLibrary.MakeRotator` 0.0 0.0 (`KismetMathLibrary.Lerp` 0.0 110.0 _alpha)) false false)))
      (else
        (`PrimitiveComponent.SetCollisionResponseToChannel` (`self.Door`) "ECC_GameTraceChannel1" "ECR_Ignore")))))

(event `EnhancedInput|/Game/Player/Input/IA_Interact`
  (params (ActionValue :type Boolean) (ElapsedSeconds :type "Float (double-precision)") (TriggeredSeconds :type "Float (double-precision)") (InputAction :type "InputAction Object Reference" :default "/Game/Player/Input/IA_Interact.IA_Interact"))
  (bind _returnvalue (`GameplayStatics.GetPlayerController` 0))
  (bind _desc_widget_ref (`self.Desc Widget Ref`))
  (:`Triggered`
    (`/Engine/EditorBlueprintResources/StandardMacros.IsValid` _desc_widget_ref
      (:`Is Valid`
        (`Widget.RemoveFromParent` _desc_widget_ref)
        (`self.DisableInput` _returnvalue)
        (`self.EnableInput` (`GameplayStatics.GetPlayerCharacter` 0) _returnvalue)
        (bind _assp_gameplay_pc (cast `/Game/SP_GameplayPC` (`GameplayStatics.GetPlayerController` 0)))
        (`/Game/SP_GameplayPC.evShowInventory` _assp_gameplay_pc)))))

(event `/Game/Blueprints/BPInterfaces/BPi_Interact.ShowHUD`
  ;[1 1 1] Show Hint Logic
  (if (`PrimitiveComponent.IsOverlappingActor` (`self.InteractionCollisionSphere`) (`GameplayStatics.GetPlayerCharacter` 0))
    (`SceneComponent.SetVisibility` (`self.innerInteractionIcon`) true false)
    (if (`self.IsMainGoal?`)
      (`SceneComponent.SetVisibility` (`self.outerInteractionIcon`) false false))
    (else
      (`SceneComponent.SetVisibility` (`self.innerInteractionIcon`) false false :!label _label)
      (if (`self.IsMainGoal?`)
        (`SceneComponent.SetVisibility` (`self.outerInteractionIcon`) true false)))))

(event `/Game/Blueprints/BPInterfaces/BPi_Interact.HideHUD`
  ;[1 1 1] Show Hint Logic
  (if (`PrimitiveComponent.IsOverlappingActor` (`self.InteractionCollisionSphere`) (`GameplayStatics.GetPlayerCharacter` 0))
    (goto _label)))

(event `self.InterestCollisionSphere.OnComponentBeginOverlap`
  (params (OverlappedComponent :type "PrimitiveComponent Object Reference") (OtherActor :type "Actor Object Reference") (OtherComp :type "PrimitiveComponent Object Reference") (OtherBodyIndex :type Integer) (bFromSweep :type Boolean) (SweepResult :type "HitResult Structure (by ref)"))
  ;[1 1 1] Show Hint Logic
  (if (and (== OtherActor (`GameplayStatics.GetPlayerCharacter` 0)) (`self.IsMainGoal?`))
    (`SceneComponent.SetVisibility` (`self.outerInteractionIcon`) true false)))

(event `self.InterestCollisionSphere.OnComponentEndOverlap`
  (params (OverlappedComponent :type "PrimitiveComponent Object Reference") (OtherActor :type "Actor Object Reference") (OtherComp :type "PrimitiveComponent Object Reference") (OtherBodyIndex :type Integer))
  ;[1 1 1] Show Hint Logic
  (if (and (`self.IsMainGoal?`) (== (`GameplayStatics.GetPlayerCharacter` 0) OtherActor))
    (`SceneComponent.SetVisibility` (`self.outerInteractionIcon`) false false)))

(fn `fnShowDescription`
  (bind _returnvalue (`GameplayStatics.GetPlayerController` 0))
  (`self.DisableInput` (`GameplayStatics.GetPlayerCharacter` 0) _returnvalue)
  (`self.EnableInput` _returnvalue)
  (`GameplayStatics.SetGamePaused` true)
  (bind _returnvalue_2 (`|CreateWidget` "/Game/UI/Interaction/W_PropDesc.W_PropDesc_C" null (`self.DescriptionWhileClosed`)))
  (bind _output_get (set `self.Desc Widget Ref` _returnvalue_2))
  (`UserWidget.AddToViewport` _output_get 0))

(fn `IsExaminable`
  (returns (IsExaminable :type Boolean))
  (return false))

(fn `IsInteractable`
  (returns (IsInteractable :type Boolean))
  (return true))

(fn `IsPickable`
  (returns (IsPickable :type Boolean))
  (return false))

(fn `UserConstructionScript`
  (bind _doorid (`self.DoorID`))
  (bind (_datatable _rowname) (break `DataTableRowHandle` _doorid))
  (`|ExecutionSequence`
    (:`then_0`
      (set `self.DoorID` _doorid)
      (bind _returnvalue (`|GetDataTableRow` _datatable _rowname)
        (:`then`
          (bind (_description _locked) (break `/Game/Blueprints/Structs/STR_Doors` _returnvalue))
          (set `self.DescriptionWhileClosed` _description)
          (set `self.KeyRequired?` _locked))))
    (:`then_1`
      (`SphereComponent.SetSphereRadius` (`self.InteractionCollisionSphere`) (`self.InteractionRadius`) true)
      (`SphereComponent.SetSphereRadius` (`self.InterestCollisionSphere`) (`self.InterestRadius`) true)
      (`SceneComponent.K2_SetRelativeLocation` (`self.innerInteractionIcon`) (`self.IconsLocation`) false false)
      (`SceneComponent.K2_SetRelativeLocation` (`self.outerInteractionIcon`) (`self.IconsLocation`) false false))
    (:`then_2`
      ;[1 1 1] Debuggin Mode
      (if (`self.Debugging?`)
        (`SceneComponent.SetVisibility` (`self.outerInteractionIcon`) true false)
        (`SceneComponent.SetVisibility` (`self.innerInteractionIcon`) true false)
        (`SceneComponent.SetVisibility` (`self.InteractionCollisionSphere`) true false)
        (`SceneComponent.SetVisibility` (`self.InterestCollisionSphere`) true false)
        (else
          (`SceneComponent.SetVisibility` (`self.outerInteractionIcon`) false false)
          (`SceneComponent.SetVisibility` (`self.innerInteractionIcon`) false false)
          (`SceneComponent.SetVisibility` (`self.InteractionCollisionSphere`) false false)
          (`SceneComponent.SetVisibility` (`self.InterestCollisionSphere`) false false))))))