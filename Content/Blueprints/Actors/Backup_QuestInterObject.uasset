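; Quest item actor that the player can inspect up close and then add to their inventory.
; Inspect moves it in front of the camera and takes over input for mouse-drag rotation and stepped zoom by wheel or M/N.
; E returns input to the player and adds the item via ACInventory, destroying it on success.
; Two overlap spheres toggle near and far prompt icons; the construction script applies mesh, scale, radii and icon placement.
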(event `self.Interact`
  (params (PlayerCharacter :type "/Game/Player/SP_PlayerCharacter Object Reference"))
  ;[1 1 1] Pick Up
)

(event `/Game/Blueprints/BPInterfaces/BPi_Interact.Inspect`
  (params (PlayerCharacter :type "/Game/Player/SP_PlayerCharacter Object Reference") (`Item Mesh` :type "StaticMesh Object Reference") (Name :type Text) (Description :type Text))
  (bind _returnvalue (`GameplayStatics.GetPlayerController` 0))
  (bind _returnvalue_2 (`GameplayStatics.GetPlayerCameraManager` 0))
  (bind _staticmesh (`self.StaticMesh`))
  (bind _returnvalue_3 (`PlayerCameraManager.GetCameraRotation` _returnvalue_2))
  ;[1 1 1] Examine
  (bind _output_get (set `self.Player Character` PlayerCharacter))
  (if (== (`/Game/Blueprints/ActorComponents/AC_Interaction.Hit Object` (`/Game/Player/SP_PlayerCharacter.AC_Interaction` PlayerCharacter)) self)
    (`self.DisableInput` _output_get _returnvalue)
    (`self.EnableInput` _returnvalue)
    (`PrimitiveComponent.SetSimulatePhysics` _staticmesh false)
    (`PrimitiveComponent.SetCollisionEnabled` _staticmesh "NoCollision")
    (bind _output_get_2 (set `/Game/Blueprints/ActorComponents/AC_Interaction.CurrentlyHeldItem` self (`/Game/Player/SP_PlayerCharacter.AC_Interaction` (`self.Player Character`))))
    (`self.K2_SetActorLocationAndRotation` _output_get_2 (+ (`PlayerCameraManager.GetCameraLocation` _returnvalue_2) (* (`KismetMathLibrary.GetForwardVector` _returnvalue_3) (`self.Inspection Distance`))) _returnvalue_3 false false)))

(event `Key|E`
  (params (Key :type "Key Structure"))
  (bind _player_character (`self.Player Character`))
  (bind (_itemid_datatable _itemid_rowname) (break `DataTableRowHandle` (`self.ItemID`)))
  (bind _ac_inventory (`/Game/Player/SP_PlayerCharacter.AC_Inventory` _player_character))
  ;[1 1 1] Actor Inputs
  (:`Pressed`
    (`self.DisableInput` (`GameplayStatics.GetPlayerController` 0))
    (`self.EnableInput` _player_character (`GameplayStatics.GetPlayerController` 0))
    (`/Engine/EditorBlueprintResources/StandardMacros.IsValid` _ac_inventory
      (:`Is Valid`
        (bind _success (`/Game/Blueprints/ActorComponents/AC_Inventory.fnAddToInventory` _ac_inventory _itemid_rowname (`self.Quantity`)))
        (if _success
          (`self.K2_DestroyActor`))))))

(event `Key|LeftMouseButton`
  (params (Key :type "Key Structure"))
  ;[1 1 1] Actor Inputs
  (:`Pressed`
    (set `self.IsRotating` true))
  (:`Released`
    (set `self.IsRotating` false)))

(event `InputAxisKey|MouseX`
  (params (AxisValue :type "Float (single-precision)"))
  ;[1 1 1] Actor Inputs
  (if (`self.IsRotating`)
    (`self.K2_SetActorRotation` (`KismetMathLibrary.ComposeRotators` (`self.K2_GetActorRotation`) (`KismetMathLibrary.MakeRotator` 0.0 0.0 (* AxisValue -5.0))))))

(event `InputAxisKey|MouseY`
  (params (AxisValue :type "Float (single-precision)"))
  ;[1 1 1] Actor Inputs
  (if (`self.IsRotating`)
    (`self.K2_SetActorRotation` (`KismetMathLibrary.ComposeRotators` (`self.K2_GetActorRotation`) (`KismetMathLibrary.MakeRotator` 0.0 (* AxisValue -5.0))))))

(event `Key|M`
  (params (Key :type "Key Structure"))
  (bind _returnvalue (`GameplayStatics.GetPlayerCameraManager` 0))
  ;[1 1 1] Actor Inputs
  (:`Pressed`
    (bind _output_get (set `self.Zoom Level` (`KismetMathLibrary.Clamp` (+ (`self.Zoom Level`) 1) (`self.Min Zoom Level`) (`self.Max Zoom Level`)) :!label _label))
    (`KismetSystemLibrary.PrintString` (`KismetStringLibrary.Conv_IntToString` _output_get))
    (if (<= _output_get (`self.Max Zoom Level`))
      (`self.K2_SetActorLocation` (+ (`PlayerCameraManager.GetCameraLocation` _returnvalue) (* (`KismetMathLibrary.GetForwardVector` (`PlayerCameraManager.GetCameraRotation` _returnvalue)) (* (`self.Zoom Level`) (`self.Zoom Multiplier`))))))))

(event `Key|MouseScrollUp`
  (params (Key :type "Key Structure"))
  ;[1 1 1] Actor Inputs
  (:`Pressed`
    (goto _label)))

(event `Key|N`
  (params (Key :type "Key Structure"))
  (bind _returnvalue (`GameplayStatics.GetPlayerCameraManager` 0))
  ;[1 1 1] Actor Inputs
  (:`Pressed`
    (bind _output_get (set `self.Zoom Level` (`KismetMathLibrary.Clamp` (- (`self.Zoom Level`) 1) (`self.Min Zoom Level`) (`self.Max Zoom Level`)) :!label _label_2))
    (`KismetSystemLibrary.PrintString` (`KismetStringLibrary.Conv_IntToString` _output_get))
    (if (>= _output_get (`self.Min Zoom Level`))
      (`self.K2_SetActorLocation` (+ (`PlayerCameraManager.GetCameraLocation` _returnvalue) (* (`KismetMathLibrary.GetForwardVector` (`PlayerCameraManager.GetCameraRotation` _returnvalue)) (* (`self.Zoom Level`) (`self.Zoom Multiplier`))))))))

(event `Key|MouseScrollDown`
  (params (Key :type "Key Structure"))
  ;[1 1 1] Actor Inputs
  (:`Pressed`
    (goto _label_2)))

(event `self.innerSphereCollision.OnComponentBeginOverlap`
  (params (OverlappedComponent :type "PrimitiveComponent Object Reference") (OtherActor :type "Actor Object Reference") (OtherComp :type "PrimitiveComponent Object Reference") (OtherBodyIndex :type Integer) (bFromSweep :type Boolean) (SweepResult :type "HitResult Structure (by ref)"))
  ;[1 1 1] Interaction Billboard Visibility
  (if (== OtherActor (`GameplayStatics.GetPlayerCharacter` 0))
    (`SceneComponent.SetVisibility` (`self.innerInteraction`) true false)
    (`SceneComponent.SetVisibility` (`self.outerInteraction`) false false)))

(event `self.innerSphereCollision.OnComponentEndOverlap`
  (params (OverlappedComponent :type "PrimitiveComponent Object Reference") (OtherActor :type "Actor Object Reference") (OtherComp :type "PrimitiveComponent Object Reference") (OtherBodyIndex :type Integer))
  ;[1 1 1] Interaction Billboard Visibility
  (if (== (`GameplayStatics.GetPlayerCharacter` 0) OtherActor)
    (`SceneComponent.SetVisibility` (`self.innerInteraction`) false false)
    (`SceneComponent.SetVisibility` (`self.outerInteraction`) true false)))

(event `self.outerSphereCollision.OnComponentBeginOverlap`
  (params (OverlappedComponent :type "PrimitiveComponent Object Reference") (OtherActor :type "Actor Object Reference") (OtherComp :type "PrimitiveComponent Object Reference") (OtherBodyIndex :type Integer) (bFromSweep :type Boolean) (SweepResult :type "HitResult Structure (by ref)"))
  ;[1 1 1] Interaction Billboard Visibility
  (if (== OtherActor (`GameplayStatics.GetPlayerCharacter` 0))
    (`SceneComponent.SetVisibility` (`self.outerInteraction`) true false)))

(event `self.outerSphereCollision.OnComponentEndOverlap`
  (params (OverlappedComponent :type "PrimitiveComponent Object Reference") (OtherActor :type "Actor Object Reference") (OtherComp :type "PrimitiveComponent Object Reference") (OtherBodyIndex :type Integer))
  ;[1 1 1] Interaction Billboard Visibility
  (if (== (`GameplayStatics.GetPlayerCharacter` 0) OtherActor)
    (`SceneComponent.SetVisibility` (`self.outerInteraction`) false false)))

(fn `IsExaminable`
  (returns (IsExaminable :type Boolean))
  (return true))

(fn `IsInteractable`
  (returns (IsInteractable :type Boolean))
  (return true))

(fn `IsPickable`
  (returns (IsPickable :type Boolean))
  (return true))

(fn `UserConstructionScript`
  (bind _staticmesh (`self.StaticMesh`))
  (`|ExecutionSequence`
    (:`then_0`
      (`SphereComponent.SetSphereRadius` (`self.outerSphereCollision`) (`self.outerInterSphereRadius`) true)
      (`SphereComponent.SetSphereRadius` (`self.innerSphereCollision`) (`self.innerInterSphereRadius`) true)
      (`SceneComponent.K2_SetRelativeLocation` (`self.innerInteraction`) (`self.IconLocation`) false false)
      (`SceneComponent.K2_SetRelativeLocation` (`self.outerInteraction`) (`self.IconLocation`) false false))
    (:`then_1`
      (`StaticMeshComponent.SetStaticMesh` (`self.StaticMesh`) (`self.Item Mesh`))
      (`SceneComponent.K2_SetWorldTransform` _staticmesh (`KismetMathLibrary.MakeTransform` (`SceneComponent.K2_GetComponentLocation` _staticmesh) (`SceneComponent.K2_GetComponentRotation` _staticmesh) (`self.Item Scale`)) false false))
    (:`then_2`
      (if (`self.Debugging?`)
        (`SceneComponent.SetVisibility` (`self.outerSphereCollision`) true false)
        (`SceneComponent.SetVisibility` (`self.innerSphereCollision`) true false)
        (else
          (`SceneComponent.SetVisibility` (`self.outerSphereCollision`) true false)
          (`SceneComponent.SetVisibility` (`self.innerSphereCollision`) true false))))))