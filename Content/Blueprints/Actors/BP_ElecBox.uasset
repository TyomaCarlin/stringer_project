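; Interactable electrical box whose door swings open once when the player interacts with it.
; A timeline drives the door pivot's yaw while the box body and door stop responding to Visibility and WorldDynamic, presumably exposing what is inside to traces.
; BeginPlay caches the BP_ElBoxTrigger and its AllLightsSwitched value, though nothing here reads them.
; The interaction queries report it as interactable, not examinable, with empty look-at text.
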(event `self.ReceiveBeginPlay`
  (bind _returnvalue (`GameplayStatics.GetActorOfClass` "/Game/Blueprints/Actors/BP_ElBoxTrigger.BP_ElBoxTrigger_C"))
  (bind _output_get (set `self.Trigger` _returnvalue))
  (set `self.All Lights Switched` (`/Game/Blueprints/Actors/BP_ElBoxTrigger.AllLightsSwitched` _output_get)))

(event `/Game/Blueprints/BPInterfaces/BPi_Interact.Interact`
  (params (PlayerCharacter :type "/Game/Characters/Player/SP_PlayerCharacter Object Reference"))
  (bind _doorpivot (`self.DoorPivot`))
  (bind (_relativerotation_roll _relativerotation_pitch) (`KismetMathLibrary.BreakRotator` (`SceneComponent.RelativeRotation` _doorpivot)))
  (`/Engine/EditorBlueprintResources/StandardMacros.DoOnce` false
    (:`Completed`
      (if (not (`self.ElBoxDoorOpen`))
        (set `self.ElBoxDoorOpen` true)
        (bind (_direction _alpha) (`Timeline|Open\\Close ElBoxDoor`)
          (:`Update`
            (`SceneComponent.K2_SetRelativeRotation` _doorpivot (`KismetMathLibrary.MakeRotator` _relativerotation_roll _relativerotation_pitch _alpha) false false)
            (`PrimitiveComponent.SetCollisionResponseToChannel` (`self.ElectricityBodyBox`) "ECC_Visibility" "ECR_Ignore")
            (`PrimitiveComponent.SetCollisionResponseToChannel` (`self.ElBoxDoor`) "ECC_Visibility" "ECR_Ignore")
            (`PrimitiveComponent.SetCollisionResponseToChannel` (`self.ElBoxDoor`) "ECC_WorldDynamic" "ECR_Ignore")
            (`PrimitiveComponent.SetCollisionResponseToChannel` (`self.ElectricityBodyBox`) "ECC_WorldDynamic" "ECR_Ignore")))))))

(fn `IsExaminable`
  (returns (IsExaminable :type Boolean))
  (return false))

(fn `IsInteractable`
  (returns (IsInteractable :type Boolean))
  (return true))

(fn `LookAt`
  (returns (Messege :type Text))
  (return ""))

(fn `UserConstructionScript`)