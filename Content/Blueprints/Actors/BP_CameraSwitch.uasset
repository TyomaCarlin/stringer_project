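; Trigger volume actor that switches the player's view between placed cameras as the SP_PlayerCharacter moves through its box.
; Entering the box sets the view target to ActiveCamera; leaving sets it to NextCamera, if valid.
; When CameraFollows is on, Tick smoothly rotates ActiveCamera toward the player with RInterpTo at DelaySpeed, whether or not the player is inside the box.
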(event `self.ReceiveTick`
  (params (DeltaSeconds :type "Float (single-precision)"))
  (bind _cameracomponent (`CameraActor.CameraComponent` (`self.Active Camera`)))
  (bind _assp_player_character (cast `/Game/Characters/Player/SP_PlayerCharacter` (`GameplayStatics.GetPlayerCharacter` 0)))
  (set `self.PlayerCharacter` _assp_player_character)
  (if (`self.CameraFollows`)
    (`SceneComponent.K2_SetWorldRotation` _cameracomponent (`KismetMathLibrary.RInterpTo` (`SceneComponent.K2_GetComponentRotation` _cameracomponent) (`KismetMathLibrary.FindLookAtRotation` (`SceneComponent.K2_GetComponentLocation` _cameracomponent) (`self.K2_GetActorLocation` (`self.PlayerCharacter`))) (`GameplayStatics.GetWorldDeltaSeconds`) (`self.Delay Speed`)) false false)))

(event `self.Box.OnComponentBeginOverlap`
  (params (OverlappedComponent :type "PrimitiveComponent Object Reference") (OtherActor :type "Actor Object Reference") (OtherComp :type "PrimitiveComponent Object Reference") (OtherBodyIndex :type Integer) (bFromSweep :type Boolean) (SweepResult :type "HitResult Structure (by ref)"))
  (bind _assp_player_character (cast `/Game/Characters/Player/SP_PlayerCharacter` OtherActor))
  (set `self.PlayerCharacter` _assp_player_character)
  (`PlayerController.SetViewTargetWithBlend` (`GameplayStatics.GetPlayerController` 0) (`self.Active Camera`) 0.0 "VTBlend_Linear" 0.0 false))

(event `self.Box.OnComponentEndOverlap`
  (params (OverlappedComponent :type "PrimitiveComponent Object Reference") (OtherActor :type "Actor Object Reference") (OtherComp :type "PrimitiveComponent Object Reference") (OtherBodyIndex :type Integer))
  (`/Engine/EditorBlueprintResources/StandardMacros.IsValid` (`self.Next Camera`)
    (:`Is Valid`
      (bind _assp_player_character (cast `/Game/Characters/Player/SP_PlayerCharacter` OtherActor))
      (set `self.PlayerCharacter` _assp_player_character)
      (`PlayerController.SetViewTargetWithBlend` (`GameplayStatics.GetPlayerController` 0) (`self.Next Camera`) 0.0 "VTBlend_Linear" 0.0 false))))

(fn `UserConstructionScript`)