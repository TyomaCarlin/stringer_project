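; Quest item pickup whose name, description, quantity and mesh are filled from a data table row in the construction script.
; Inner and outer spheres, sized per instance, drive near and far interaction icons.
; Interacting, if inspectable, spawns BP_InspectItem far off in the world, adds the item to the player's inventory and opens first-time inspection.
; On destruction it registers itself in the game mode's level save data as removed.
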(event `self.ReceiveDestroyed`
  ;[1 1 1] Save Destroyed QItems in Level
  (bind _assp_gameplay_gm (cast `/Game/SP_GameplayGM` (`GameplayStatics.GetGameMode`)))
  (`KismetArrayLibrary.Array_AddUnique` (`/Game/SaveData/SaveData_L_Start.ActorRemoved` (`/Game/SP_GameplayGM.Save Data Level` _assp_gameplay_gm)) (`|ConvertAsset` self)))

(event `/Game/Blueprints/BPInterfaces/BPi_Interact.Interact`
  (params (PlayerCharacter :type "/Game/Player/SP_PlayerCharacter Object Reference"))
  (bind (_itemid_datatable _itemid_rowname) (break `DataTableRowHandle` (`self.ItemID`)))
  (bind _ac_inventorie (`/Game/Player/SP_PlayerCharacter.AC_Inventorie` PlayerCharacter))
  ;[1 1 1] Interaction
  (`|ExecutionSequence`
    (:`then_0`
      (if (== (`/Game/Blueprints/ActorComponents/AC_Interaction.Hit Object` (`/Game/Player/SP_PlayerCharacter.AC_Interaction` PlayerCharacter)) self)
        (if (`self.Inspectable?`)
          (bind _returnvalue (`|SpawnActorFromClass` "/Game/Blueprints/Actors/BP_InspectItem.BP_InspectItem_C" (`KismetMathLibrary.MakeTransform` (100000000.0 0.0 0.0)) "Undefined" "MultiplyWithRoot" null null))
          (`/Game/Blueprints/Actors/BP_InspectItem.evSetInspectRotation` _returnvalue (`self.Inspection Rotation`))
          (`/Game/Blueprints/Actors/BP_InspectItem.evSetInspectScale` _returnvalue (`self.Inspection Scale`))
          (`/Engine/EditorBlueprintResources/StandardMacros.IsValid` _ac_inventorie
            (:`Is Valid`
              (`/Game/Blueprints/ActorComponents/AC_Inventorie.fnAdd` _ac_inventorie _itemid_rowname (`self.Quantity`))
              (message `/Game/Blueprints/BPInterfaces/BPi_Interact.Inspect` _returnvalue PlayerCharacter (`StaticMeshComponent.StaticMesh` (`self.StaticMesh`)) (`self.Item Name`) (`self.Item Description`) self false true))))))))

(event `/Game/Blueprints/BPInterfaces/BPi_Interact.ShowHUD`
  ;[1 1 1] Show Hint Logic
  (if (`PrimitiveComponent.IsOverlappingActor` (`self.innerSphereCollision`) (`GameplayStatics.GetPlayerCharacter` 0))
    (`SceneComponent.SetVisibility` (`self.innerInteractionIcon`) true false)
    (`SceneComponent.SetVisibility` (`self.outerInteractionIcon`) false false)
    (else
      (`SceneComponent.SetVisibility` (`self.innerInteractionIcon`) false false :!label _label)
      (`SceneComponent.SetVisibility` (`self.outerInteractionIcon`) true false))))

(event `/Game/Blueprints/BPInterfaces/BPi_Interact.HideHUD`
  ;[1 1 1] Show Hint Logic
  (if (`PrimitiveComponent.IsOverlappingActor` (`self.innerSphereCollision`) (`GameplayStatics.GetPlayerCharacter` 0))
    (goto _label)))

(event `self.outerSphereCollision.OnComponentBeginOverlap`
  (params (OverlappedComponent :type "PrimitiveComponent Object Reference") (OtherActor :type "Actor Object Reference") (OtherComp :type "PrimitiveComponent Object Reference") (OtherBodyIndex :type Integer) (bFromSweep :type Boolean) (SweepResult :type "HitResult Structure (by ref)"))
  ;[1 1 1] Show Hint Logic
  (if (== OtherActor (`GameplayStatics.GetPlayerCharacter` 0))
    (`SceneComponent.SetVisibility` (`self.outerInteractionIcon`) true false)))

(event `self.outerSphereCollision.OnComponentEndOverlap`
  (params (OverlappedComponent :type "PrimitiveComponent Object Reference") (OtherActor :type "Actor Object Reference") (OtherComp :type "PrimitiveComponent Object Reference") (OtherBodyIndex :type Integer))
  ;[1 1 1] Show Hint Logic
  (if (== (`GameplayStatics.GetPlayerCharacter` 0) OtherActor)
    (`SceneComponent.SetVisibility` (`self.outerInteractionIcon`) false false)))

(fn `IsExaminable`
  (returns (IsExaminable :type Boolean))
  (return true))

(fn `IsInteractable`
  (returns (IsInteractable :type Boolean))
  (return true))

(fn `IsPickable`
  (returns (IsPickable :type Boolean))
  (return true))

(fn `UserConstructionScript`
  (bind _staticmesh (`self.StaticMesh`))
  (`|ExecutionSequence`
    (:`then_0`
      (bind _output_get (set `self.ItemID` (`self.ItemID`)))
      (bind (_datatable _rowname) (break `DataTableRowHandle` _output_get))
      (bind _returnvalue (`|GetDataTableRow` _datatable _rowname)
        (:`then`
          (bind (_name _description _mesh _itemactor _thumbnail _stacksize) (break `/Game/Blueprints/Structs/STR_QuestItems` _returnvalue))
          (set `self.Item Name` _name)
          (set `self.Item Description` _description)
          (set `self.Quantity` _stacksize))))
    (:`then_1`
      (`SphereComponent.SetSphereRadius` (`self.outerSphereCollision`) (`self.outerInterSphereRadius`) true)
      (`SphereComponent.SetSphereRadius` (`self.innerSphereCollision`) (`self.innerInterSphereRadius`) true)
      (`SceneComponent.K2_SetRelativeLocation` (`self.innerInteractionIcon`) (`self.IconLocation`) false false)
      (`SceneComponent.K2_SetRelativeLocation` (`self.outerInteractionIcon`) (`self.IconLocation`) false false))
    (:`then_2`
      ;[1 1 1] Setting Mesh Dynamically
      (`StaticMeshComponent.SetStaticMesh` (`self.StaticMesh`) _mesh)
      ;[1 1 1] Setting Scale of the Mesh Dynamically
      (`SceneComponent.K2_SetWorldTransform` _staticmesh (`KismetMathLibrary.MakeTransform` (`SceneComponent.K2_GetComponentLocation` _staticmesh) (`SceneComponent.K2_GetComponentRotation` _staticmesh) (`self.Item Scale`)) false false))
    (:`then_3`
      ;[1 1 1] Debuggin Mode
      (if (`self.Debugging?`)
        (`SceneComponent.SetVisibility` (`self.outerSphereCollision`) true false)
        (`SceneComponent.SetVisibility` (`self.innerSphereCollision`) true false)
        (`SceneComponent.SetVisibility` (`self.outerInteractionIcon`) true false)
        (`SceneComponent.SetVisibility` (`self.innerInteractionIcon`) true false)
        (else
          (`SceneComponent.SetVisibility` (`self.outerSphereCollision`) false false)
          (`SceneComponent.SetVisibility` (`self.innerSphereCollision`) false false)
          (`SceneComponent.SetVisibility` (`self.outerInteractionIcon`) false false)
          (`SceneComponent.SetVisibility` (`self.innerInteractionIcon`) false false))))))