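; BP_Notes is an interactable note actor that the player can open and close to read.
; Its Interact event toggles an IsReading flag, copying NoteDescription into the player character's Note and showing the WBNote widget on MasterUI, or collapsing it on the next interaction.
; IsInteractable always returns true; the other events are unused stubs.
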(event `/Game/Blueprints/BPInterfaces/BPi_Interact.Interact`
  (params (PlayerCharacter :type "/Game/Characters/Player/SP_PlayerCharacter Object Reference"))
  (bind _wb_note (`/Game/UI/WB_MasterUI.WB_Note` (`/Game/Characters/Player/SP_PlayerCharacter.MasterUI` PlayerCharacter)))
  (if (`self.IsReading`)
    (`Widget.SetVisibility` _wb_note "Collapsed")
    (set `self.IsReading` false)
    (else
      (set `/Game/Characters/Player/SP_PlayerCharacter.Note` (`self.NoteDescription`) PlayerCharacter)
      (`Widget.SetVisibility` _wb_note "Visible")
      (set `self.IsReading` true))))

(fn `IsInteractable`
  (returns (IsInteractable :type Boolean))
  (return true))

(fn `UserConstructionScript`
  (`parent.UserConstructionScript`))