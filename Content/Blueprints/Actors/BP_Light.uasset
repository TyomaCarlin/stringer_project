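; BP_Light is a configurable light actor whose on/off state and appearance are set from its variables.
; The construction script shows or hides the LightSource component according to IsLightOn, then applies intensity, units, attenuation radius and color.
; Separate turn-on and turn-off functions update the IsLightOn flag together with the component's visibility.
; The event graph holds only disabled placeholder events, so the actor runs no per-frame or BeginPlay logic.
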(fn `fnTurnOffLight`
  (set `self.IsLightOn?` false)
  (`SceneComponent.SetVisibility` (`self.LightSource`) false false))

(fn `fnTurnOnLight`
  (set `self.IsLightOn?` true)
  (`SceneComponent.SetVisibility` (`self.LightSource`) true false))

(fn `UserConstructionScript`
  (bind _lightsource (`self.LightSource`))
  (if (`self.IsLightOn?`)
    (`self.fnTurnOnLight`)
    (else
      (`self.fnTurnOffLight`)))
  (`LightComponent.SetIntensity` _lightsource (`self.LightIntensity`))
  (`LocalLightComponent.SetIntensityUnits` _lightsource (`self.LightIntensityUnits`))
  (`LocalLightComponent.SetAttenuationRadius` _lightsource (`self.LightRadius`))
  (`LightComponent.SetLightColor` _lightsource (`self.LightColor`) true))