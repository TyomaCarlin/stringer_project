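; BP_PillarButton1 is an interactable, non-examinable pillar button that moves vertically and signals when activated.
; Start drives its world Z from a timeline, then sets the cube to block a game trace channel when the move finishes.
; Interact sets IsActivated, fires the ButtonActivated dispatcher and plays the MoveDown timeline, whose curve sets absolute Z.
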(event `/Game/Blueprints/BPInterfaces/BPi_Triggerable.Start`
  (bind (_returnvalue_x _returnvalue_y) (`KismetMathLibrary.BreakVector` (`self.K2_GetActorLocation`)))
  (bind (_direction _alpha) (`Timeline|Timeline`)
    (:`Update`
      (`self.K2_SetActorLocation` (`KismetMathLibrary.MakeVector` _returnvalue_x _returnvalue_y _alpha)))
    (:`Finished`
      (`PrimitiveComponent.SetCollisionResponseToChannel` (`self.Cube`) "ECC_GameTraceChannel1" "ECR_Block"))))

(event `/Game/Blueprints/BPInterfaces/BPi_Interact.Interact`
  (params (PlayerCharacter :type "/Game/Characters/Player/SP_PlayerCharacter Object Reference"))
  (bind (_returnvalue_x _returnvalue_y) (`KismetMathLibrary.BreakVector` (`self.K2_GetActorLocation` self)))
  (`KismetSystemLibrary.PrintString` "Button Interacted")
  (set `self.IsActivated` true)
  (`self.ButtonActivated`)
  (`KismetSystemLibrary.PrintString` "Dispatcher Called")
  (bind (_direction _alpha) (`Timeline|Move Down`)
    (:`Update`
      (`self.K2_SetActorLocation` self (`KismetMathLibrary.MakeVector` _returnvalue_x _returnvalue_y _alpha) false false))))

(fn `IsExaminable`
  (returns (IsExaminable :type Boolean))
  (return false))

(fn `IsInteractable`
  (returns (IsInteractable :type Boolean))
  (return true))

(fn `LookAt`
  (returns (Messege :type Text))
  (return ""))

(fn `UserConstructionScript`)