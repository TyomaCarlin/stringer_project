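; BP_ItemEffect is an actor that applies an item's effect as soon as it begins play, currently changing a door's key requirement.
; When flagged as a key, it searches all BP_Doors1 actors for a DoorID row name matching its TargetID.
; It sets the matched door's KeyRequired to its DoorLockState value.
; It then destroys itself if WillBeDestroyed is set, whether or not it is a key.
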(event `self.ReceiveBeginPlay`
  (bind (_targetid_datatable _targetid_rowname) (break `DataTableRowHandle` (`self.TargetID`)))
  (bind (_asbp_doors_1 _bsuccess) (cast `/Game/Blueprints/Actors/BP_Doors1` (`self.TargetActor`) :!pure true))
  (`|ExecutionSequence`
    (:`then_0`
      (if (`self.IsKey?`)
        (`|ExecutionSequence`
          (:`then_0`
            (bind _outactors (`GameplayStatics.GetAllActorsOfClass` "/Game/Blueprints/Actors/BP_Doors1.BP_Doors1_C"))
            (for _array_element _outactors
              (bind (_doorid_datatable _doorid_rowname) (break `DataTableRowHandle` (`/Game/Blueprints/Actors/BP_Doors1.DoorID` _array_element)))
              (if (== _doorid_rowname _targetid_rowname)
                (set `self.TargetActor` _array_element))))
          (:`then_1`
            (if _bsuccess
              (set `/Game/Blueprints/Actors/BP_Doors1.KeyRequired?` (`self.DoorLockState`) _asbp_doors_1))))))
    (:`then_1`
      (if (`self.WillBeDestroyed?`)
        (`self.K2_DestroyActor`)))))

(fn `UserConstructionScript`)