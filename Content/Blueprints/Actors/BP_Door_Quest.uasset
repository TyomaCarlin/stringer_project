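; Quest door actor that swings open on interaction, or requires a matching key item while locked.
; Interacting while locked opens the player's inventory through SP_GameplayPC; using an item whose ID matches RequiredKeyID unlocks and opens the door.
; Opening plays a timeline that lerps the Pivot's yaw, with no closing logic.
; The locked-feedback event for a wrong item is an empty stub.
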(event `evOpenDoor`
  (bind (_direction _alpha) (`Timeline|Timeline`)
    (:`Update`
      (`SceneComponent.K2_SetRelativeRotation` (`self.Pivot`) (`KismetMathLibrary.MakeRotator` 0.0 0.0 (`KismetMathLibrary.Lerp` 0.0 110.0 _alpha)) false false))))

(event `/Game/Blueprints/Interfaces/BPI_Interactable.OnInteract`
  (params (Interactor :type "Actor Object Reference"))
  (if (`self.bIsLocked`)
    (bind _assp_gameplay_pc (cast `/Game/SP_GameplayPC` (`GameplayStatics.GetPlayerController` 0)))
    (`/Game/SP_GameplayPC.evShowInventory` _assp_gameplay_pc)
    (else
      (`self.evOpenDoor`))))

(event `/Game/Blueprints/Interfaces/BPI_Interactable.OnUseItem`
  (params (Item :type "/Game/Blueprints/Actors/BP_ItemBase Object Reference"))
  (if (== (`/Game/Blueprints/Actors/BP_ItemBase.ItemID` Item) (`self.RequiredKeyID`))
    (set `self.bIsLocked` false)
    (`self.evOpenDoor`)
    (else
      (`self.evPlayLockedFeedback`))))

(event `evPlayLockedFeedback`)

(fn `UserConstructionScript`)