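; BP_Note is an interactable, non-pickable note that the player reads up close.
; The construction script loads text and mesh from a data table row and configures triggers, hint icons, camera and debug visibility.
; Interacting blends to the note's view, opens W_InspectNote, moves input to the note and freezes time until closed, with IA_R toggling extra text.
; Inner and outer spheres drive interact and quest-interest hints, the latter only for main quest goals.
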(event `/Game/Blueprints/BPInterfaces/BPi_Interact.Interact`
  (params (PlayerCharacter :type "/Game/Player/SP_PlayerCharacter Object Reference"))
  (bind _returnvalue (`GameplayStatics.GetPlayerController` 0))
  (set `self.InspectingNote` true)
  (`|ExecutionSequence`
    (:`then_0`
      (if (== (`/Game/Blueprints/ActorComponents/AC_Interaction.Hit Object` (`/Game/Player/SP_PlayerCharacter.AC_Interaction` PlayerCharacter)) self)
        (`PlayerController.SetViewTargetWithBlend` (`GameplayStatics.GetPlayerController` 0) self 0.0 "VTBlend_Linear" 0.0 false)))
    (:`then_1`
      (set `/Game/SP_GameplayPC.InspectingItem?` true (cast `/Game/SP_GameplayPC` (`GameplayStatics.GetPlayerController` 0) :!pure true))
      (bind _returnvalue_2 (`|CreateWidget` "/Game/UI/Interaction/W_InspectNote.W_InspectNote_C" null (`self.NoteText`)))
      (bind _output_get (set `self.Note Widget Ref` _returnvalue_2))
      (`UserWidget.AddToViewport` _output_get 0)
      (`self.DisableInput` (`GameplayStatics.GetPlayerCharacter` 0) _returnvalue)
      (`self.EnableInput` _returnvalue)
      (`KismetSystemLibrary.Delay` 0.2)
      (`GameplayStatics.SetGlobalTimeDilation` 0.0))))

(event `EnhancedInput|/Game/Player/Input/IA_Interact`
  (params (ActionValue :type Boolean) (ElapsedSeconds :type "Float (double-precision)") (TriggeredSeconds :type "Float (double-precision)") (InputAction :type "InputAction Object Reference" :default "/Game/Player/Input/IA_Interact.IA_Interact"))
  (bind _returnvalue (`GameplayStatics.GetPlayerController` 0))
  (bind _note_widget_ref (`self.Note Widget Ref`))
  (:`Triggered`
    (`/Engine/EditorBlueprintResources/StandardMacros.IsValid` _note_widget_ref
      (:`Is Valid`
        (`Widget.RemoveFromParent` _note_widget_ref)
        (set `self.Note Widget Ref` null)
        (`self.DisableInput` _returnvalue)
        (`self.EnableInput` (`GameplayStatics.GetPlayerCharacter` 0) _returnvalue)
        (bind _assp_gameplay_pc (cast `/Game/SP_GameplayPC` (`GameplayStatics.GetPlayerController` 0)))
        (set `/Game/SP_GameplayPC.InspectingItem?` false _assp_gameplay_pc)
        (set `self.InspectingNote` false)
        (`self.Check`)
        (`GameplayStatics.SetGlobalTimeDilation` 1.0)
        (`PlayerController.SetViewTargetWithBlend` (`GameplayStatics.GetPlayerController` 0) (`self.CameraToLeave`) 0.0 "VTBlend_Linear" 0.0 false)))))

(event `EnhancedInput|/Game/Player/Input/IA_R`
  (params (ActionValue :type Boolean) (ElapsedSeconds :type "Float (double-precision)") (TriggeredSeconds :type "Float (double-precision)") (InputAction :type "InputAction Object Reference" :default "/Game/Player/Input/IA_R.IA_R"))
  (bind _brd_text (`/Game/UI/Interaction/W_InspectNote.BRD_Text` (`self.Note Widget Ref`)))
  (:`Completed`
    (`/Engine/EditorBlueprintResources/StandardMacros.FlipFlop`
      (:`A`
        (`Widget.SetVisibility` _brd_text "Visible"))
      (:`B`
        (`Widget.SetVisibility` _brd_text "Hidden")))))

(event `/Game/Blueprints/BPInterfaces/BPi_Interact.ShowHUD`
  ;[1 1 1] Show Hint Logic
  (if (`PrimitiveComponent.IsOverlappingActor` (`self.InnerTriggerArea`) (`GameplayStatics.GetPlayerCharacter` 0))
    (`|ExecutionSequence`
      (:`then_0`
        (if (`self.IsMainQuestGoal?`)
          (`SceneComponent.SetVisibility` (`self.InterestHint`) false false)))
      (:`then_1`
        (if (not (`self.InspectingNote`))
          (`SceneComponent.SetVisibility` (`self.InteractHint`) true false))))
    (else
      (`SceneComponent.SetVisibility` (`self.InteractHint`) false false :!label _label)
      (if (and (not (`self.InspectingNote`)) (`self.IsMainQuestGoal?`))
        (`SceneComponent.SetVisibility` (`self.InterestHint`) true false)))))

(event `/Game/Blueprints/BPInterfaces/BPi_Interact.HideHUD`
  ;[1 1 1] Show Hint Logic
  (if (`PrimitiveComponent.IsOverlappingActor` (`self.InnerTriggerArea`) (`GameplayStatics.GetPlayerCharacter` 0))
    (goto _label)))

(event `self.OuterTriggerArea.OnComponentBeginOverlap`
  (params (OverlappedComponent :type "PrimitiveComponent Object Reference") (OtherActor :type "Actor Object Reference") (OtherComp :type "PrimitiveComponent Object Reference") (OtherBodyIndex :type Integer) (bFromSweep :type Boolean) (SweepResult :type "HitResult Structure (by ref)"))
  ;[1 1 1] Show Hint Logic
  (if (and (== OtherActor (`GameplayStatics.GetPlayerCharacter` 0)) (not (`self.InspectingNote`)) (`self.IsMainQuestGoal?`))
    (`SceneComponent.SetVisibility` (`self.InterestHint`) true false)))

(event `self.OuterTriggerArea.OnComponentEndOverlap`
  (params (OverlappedComponent :type "PrimitiveComponent Object Reference") (OtherActor :type "Actor Object Reference") (OtherComp :type "PrimitiveComponent Object Reference") (OtherBodyIndex :type Integer))
  ;[1 1 1] Show Hint Logic
  (if (and (== (`GameplayStatics.GetPlayerCharacter` 0) OtherActor) (`self.IsMainQuestGoal?`))
    (`SceneComponent.SetVisibility` (`self.InterestHint`) false false)))

(fn `IsExaminable`
  (returns (IsExaminable :type Boolean))
  (return false))

(fn `IsInteractable`
  (returns (IsInteractable :type Boolean))
  (return true))

(fn `IsPickable`
  (returns (IsPickable :type Boolean))
  (return false))

(fn `UserConstructionScript`
  (bind _notemesh (`self.NoteMesh`))
  (bind (_datatable _rowname) (break `DataTableRowHandle` (`self.NoteID`)))
  (`|ExecutionSequence`
    (:`then_0`
      (bind _returnvalue (`|GetDataTableRow` _datatable _rowname)
        (:`then`
          (bind (_text _mesh) (break `/Game/Blueprints/Structs/STR_Notes` _returnvalue))
          (set `self.NoteText` _text))))
    (:`then_1`
      (`SphereComponent.SetSphereRadius` (`self.OuterTriggerArea`) (`self.OuterTriggerRadius`) true)
      (`SphereComponent.SetSphereRadius` (`self.InnerTriggerArea`) (`self.InnerTriggerRadius`) true)
      (`SceneComponent.K2_SetRelativeLocation` (`self.InteractHint`) (`self.InteractIconLocation`) false false)
      (`SceneComponent.K2_SetRelativeLocation` (`self.InterestHint`) (`self.InteractIconLocation`) false false))
    (:`then_2`
      ;[1 1 1] Setting Mesh Dynamically
      (`StaticMeshComponent.SetStaticMesh` (`self.NoteMesh`) _mesh)
      ;[1 1 1] Setting Scale of the Mesh Dynamically
      (`SceneComponent.K2_SetWorldTransform` _notemesh (`KismetMathLibrary.MakeTransform` (`SceneComponent.K2_GetComponentLocation` _notemesh) (`SceneComponent.K2_GetComponentRotation` _notemesh) (`self.MeshScale`)) false false))
    (:`then_3`
      ;[1 1 1] Debuggin Mode
      (if (`self.Debugging`)
        (`SceneComponent.SetVisibility` (`self.InnerTriggerArea`) true false)
        (`SceneComponent.SetVisibility` (`self.OuterTriggerArea`) true false)
        (`SceneComponent.SetVisibility` (`self.InterestHint`) true false)
        (`SceneComponent.SetVisibility` (`self.InteractHint`) true false)
        (`SceneComponent.SetVisibility` (`self.NoteCamera`) true false)
        (else
          (`SceneComponent.SetVisibility` (`self.OuterTriggerArea`) false false)
          (`SceneComponent.SetVisibility` (`self.InnerTriggerArea`) false false)
          (`SceneComponent.SetVisibility` (`self.InteractHint`) false false)
          (`SceneComponent.SetVisibility` (`self.InterestHint`) false false)
          (`SceneComponent.SetVisibility` (`self.NoteCamera`) false false))))
    (:`then_4`
      ;[1 1 1] Camera SetUp
      (set `self.Note Camera` (`self.NoteCamera`))
      (`SceneComponent.K2_SetRelativeLocation` (`self.NoteCamera`) (`self.Location`) false false)
      (`SceneComponent.K2_SetWorldRotation` (`self.NoteCamera`) (`self.Rotation`) false false))))