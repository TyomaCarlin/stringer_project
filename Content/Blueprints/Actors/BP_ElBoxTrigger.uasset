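; BP_ElBoxTrigger is an interactable, non-examinable lever or switch that controls electricity for the level's electric box and lights.
; On BeginPlay it caches the BP_ElecBox actor.
; Each interaction flips every BP_Light individually, toggles the box's HasElectricity and plays or reverses a Timeline that rolls the Pivot.
; A DoOnce blocks repeat interactions until the Timeline finishes.
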(event `self.ReceiveBeginPlay`
  (bind _returnvalue (`GameplayStatics.GetActorOfClass` "/Game/Blueprints/Actors/BP_ElecBox.BP_ElecBox_C"))
  (set `self.ElBox` _returnvalue))

(event `/Game/Blueprints/BPInterfaces/BPi_Interact.Interact`
  (params (PlayerCharacter :type "/Game/Characters/Player/SP_PlayerCharacter Object Reference"))
  (bind _pivot (`self.Pivot`))
  (bind _elbox (`self.ElBox`))
  (bind (_relativerotation_roll _relativerotation_pitch _relativerotation_yaw) (`KismetMathLibrary.BreakRotator` (`SceneComponent.RelativeRotation` _pivot)))
  (`/Engine/EditorBlueprintResources/StandardMacros.DoOnce` false :!label _label
    (:`Completed`
      (`self.AllLightSwitch`)
      (if (not (`self.IsPulled`))
        (set `self.IsPulled` true)
        (set `/Game/Blueprints/Actors/BP_ElecBox.HasElectricity` true _elbox)
        (bind (_direction _newtrack_0) (`Timeline|Timeline` :!label _label_2)
          (:`Update`
            (`SceneComponent.K2_SetRelativeRotation` _pivot (`KismetMathLibrary.MakeRotator` _newtrack_0 _relativerotation_pitch _relativerotation_yaw) false false))
          (:`Finished`
            (goto _label :!via `Reset`)))
        (else
          (set `self.IsPulled` false)
          (set `/Game/Blueprints/Actors/BP_ElecBox.HasElectricity` false _elbox)
          (goto _label_2 :!via `Reverse`))))))

(event `AllLightSwitch`
  (bind _outactors (`GameplayStatics.GetAllActorsOfClass` "/Game/Blueprints/Actors/BP_Light.BP_Light_C"))
  (bind _output_get (set `self.AllLightsSwitched` _outactors))
  (for _array_element _output_get
    (if (`/Game/Blueprints/Actors/BP_Light.IsLightOn?` _array_element)
      (`/Game/Blueprints/Actors/BP_Light.fnTurnOffLight` _array_element)
      (else
        (`/Game/Blueprints/Actors/BP_Light.fnTurnOnLight` _array_element)))))

(fn `IsExaminable`
  (returns (IsExaminable :type Boolean))
  (return false))

(fn `IsInteractable`
  (returns (IsInteractable :type Boolean))
  (return true))

(fn `LookAt`
  (returns (Messege :type Text))
  (return ""))

(fn `UserConstructionScript`)