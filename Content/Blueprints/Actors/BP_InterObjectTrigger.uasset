(event `self.ReceiveBeginPlay`
  (if (`self.StartsActive?`)
    (`self.fnInteractionOn`)
    (else
      (`self.fnInteractionOff`))))

(event `/Game/Blueprints/BPInterfaces/BPI_FlowControl.Turn On`
  (`self.fnInteractionOn`))

(event `/Game/Blueprints/BPInterfaces/BPI_FlowControl.Turn Off`
  (`self.fnInteractionOff`))

(event `/Game/Blueprints/BPInterfaces/BPi_Interact.Interact`
  (params (PlayerCharacter :type "/Game/Player/SP_PlayerCharacter Object Reference"))
  (`self.dspCheckTriggered`))

(event `/Game/Blueprints/BPInterfaces/BPi_Interact.ShowHUD`
  ;[1 1 1] Show Hint Logic
  (if (`PrimitiveComponent.IsOverlappingActor` (`self.innerSphereCollision`) (`GameplayStatics.GetPlayerCharacter` 0))
    (`SceneComponent.SetVisibility` (`self.innerInteractionIcon`) true false)
    (if (`self.IsMainGoal?`)
      (`SceneComponent.SetVisibility` (`self.outerInteractionIcon`) false false))
    (else
      (`SceneComponent.SetVisibility` (`self.innerInteractionIcon`) false false :!label _label)
      (if (`self.IsMainGoal?`)
        (`SceneComponent.SetVisibility` (`self.outerInteractionIcon`) true false)))))

(event `/Game/Blueprints/BPInterfaces/BPi_Interact.HideHUD`
  ;[1 1 1] Show Hint Logic
  (if (`PrimitiveComponent.IsOverlappingActor` (`self.innerSphereCollision`) (`GameplayStatics.GetPlayerCharacter` 0))
    (goto _label)))

(event `self.outerSphereCollision.OnComponentBeginOverlap`
  (params (OverlappedComponent :type "PrimitiveComponent Object Reference") (OtherActor :type "Actor Object Reference") (OtherComp :type "PrimitiveComponent Object Reference") (OtherBodyIndex :type Integer) (bFromSweep :type Boolean) (SweepResult :type "HitResult Structure (by ref)"))
  ;[1 1 1] Show Hint Logic
  (if (and (== OtherActor (`GameplayStatics.GetPlayerCharacter` 0)) (`self.IsMainGoal?`))
    (`SceneComponent.SetVisibility` (`self.innerInteractionIcon`) true false)))

(event `self.outerSphereCollision.OnComponentEndOverlap`
  (params (OverlappedComponent :type "PrimitiveComponent Object Reference") (OtherActor :type "Actor Object Reference") (OtherComp :type "PrimitiveComponent Object Reference") (OtherBodyIndex :type Integer))
  ;[1 1 1] Show Hint Logic
  (if (and (`self.IsMainGoal?`) (== (`GameplayStatics.GetPlayerCharacter` 0) OtherActor))
    (`SceneComponent.SetVisibility` (`self.outerInteractionIcon`) false false)))

(fn `fnInteractionOff`
  (`PrimitiveComponent.SetCollisionResponseToChannel` (`self.StaticMesh`) "ECC_GameTraceChannel1" "ECR_Ignore")
  (`PrimitiveComponent.SetCollisionEnabled` (`self.innerSphereCollision`) "NoCollision")
  (`PrimitiveComponent.SetCollisionEnabled` (`self.outerSphereCollision`) "NoCollision")
  (`SceneComponent.SetHiddenInGame` (`self.innerInteractionIcon`) true false)
  (`SceneComponent.SetHiddenInGame` (`self.outerInteractionIcon`) true false))

(fn `fnInteractionOn`
  (`PrimitiveComponent.SetCollisionResponseToChannel` (`self.StaticMesh`) "ECC_GameTraceChannel1" "ECR_Block")
  (`PrimitiveComponent.SetCollisionEnabled` (`self.outerSphereCollision`) "QueryOnly")
  (`PrimitiveComponent.SetCollisionEnabled` (`self.innerSphereCollision`) "QueryOnly")
  (`SceneComponent.SetHiddenInGame` (`self.innerInteractionIcon`) false false)
  (`SceneComponent.SetHiddenInGame` (`self.outerInteractionIcon`) false false))

(fn `IsExaminable`
  (returns (IsExaminable :type Boolean))
  (return false))

(fn `IsInteractable`
  (returns (IsInteractable :type Boolean))
  (return false))

(fn `IsPickable`
  (returns (IsPickable :type Boolean))
  (return false))

(fn `UserConstructionScript`
  (bind _staticmesh (`self.StaticMesh`))
  (`|ExecutionSequence`
    (:`then_0`
      (bind _output_get (set `self.ItemMesh` (`self.ItemMesh`)))
      (`StaticMeshComponent.SetStaticMesh` _staticmesh _output_get)
      (if (`self.MeshHidden?`)
        (`SceneComponent.SetHiddenInGame` _staticmesh true false)
        (`PrimitiveComponent.SetCollisionResponseToAllChannels` _staticmesh "ECR_Ignore")
        (`PrimitiveComponent.SetCollisionResponseToChannel` _staticmesh "ECC_GameTraceChannel1" "ECR_Block")
        (else
          (`SceneComponent.SetHiddenInGame` _staticmesh false false)
          (`PrimitiveComponent.SetCollisionResponseToAllChannels` _staticmesh "ECR_Block"))))
    (:`then_1`
      (`SphereComponent.SetSphereRadius` (`self.outerSphereCollision`) (`self.InterestSphereRadius`) true)
      (`SphereComponent.SetSphereRadius` (`self.innerSphereCollision`) (`self.InteractSphereRadius`) true)
      (`SceneComponent.K2_SetRelativeLocation` (`self.innerInteractionIcon`) (`self.IconLocation`) false false)
      (`SceneComponent.K2_SetRelativeLocation` (`self.outerInteractionIcon`) (`self.IconLocation`) false false))
    (:`then_2`
      ;[1 1 1] Debuggin Mode
      (if (`self.Debugging?`)
        (`SceneComponent.SetVisibility` (`self.outerSphereCollision`) true false)
        (`SceneComponent.SetVisibility` (`self.innerSphereCollision`) true false)
        (`SceneComponent.SetVisibility` (`self.innerInteractionIcon`) true false)
        (`SceneComponent.SetVisibility` (`self.outerInteractionIcon`) true false)
        (else
          (`SceneComponent.SetVisibility` (`self.outerSphereCollision`) false false)
          (`SceneComponent.SetVisibility` (`self.innerSphereCollision`) false false)
          (`SceneComponent.SetVisibility` (`self.innerInteractionIcon`) false false)
          (`SceneComponent.SetVisibility` (`self.outerInteractionIcon`) false false))))))