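; Interactable trigger prop that shows up to three description lines, can grant a quest item, and can switch to an inspect camera.
; Construction fills mesh and texts from a data table row.
; Interact pauses the game with a description widget; gates and a counter route input through lines, empty or additional text, then repeat, disable or destroy.
; Overlap spheres drive hint icons, and granted items enter inventory and open BP_InspectItem.
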(event `self.ReceiveBeginPlay`
  ;[1 1 1] Begin Play
  (if (`self.StartsActive?`)
    (`self.fnInteractionOn`)
    (else
      (`self.fnInteractionOff`))))

(event `self.Turn On`
  ;[1 1 1] Turn On
  (`self.fnInteractionOn`))

(event `self.Turn Off`
  ;[1 1 1] Turn Off
  (`self.fnInteractionOff`))

(event `self.Reset Desc Inter Object`
  (params (`Gives Quest Object?` :type Boolean) (`Is Desctroyed After?` :type Boolean) (`IsMainGoal?` :type Boolean) (`Has Desc1?` :type Boolean) (`Has Desc2?` :type Boolean) (`Has Desc3?` :type Boolean) (`Has Empty Desc?` :type Boolean) (`Is Repeatable Desc?` :type Boolean) (`Has Additional Desc?` :type Boolean) (`Has Inspect view?` :type Boolean))
  ;[1 1 1] Reset
  (`|ExecutionSequence`
    (:`then_0`
      (set `self.GivesQuestObject?` `Gives Quest Object?`)
      (set `self.IsDestroyedAfter?` `Is Desctroyed After?`)
      (set `self.IsMainGoal?` `IsMainGoal?`))
    (:`then_1`
      (set `self.HasDesc1` `Has Desc1?`)
      (set `self.HasDesc2` `Has Desc2?`)
      (set `self.HasDesc3` `Has Desc3?`)
      (set `self.HasEmptyDesc?` `Has Empty Desc?`)
      (set `self.RepeatableDesc?` `Is Repeatable Desc?`)
      (set `self.HasAdditionalDesc?` `Has Additional Desc?`))
    (:`then_2`
      (set `self.HasInspectView` `Has Inspect view?`))
    (:`then_3`
      (`self.fnInteractionOn`))))

(event `evOpenAddDescGate`
  ;[1 1 1] Additional Desc
  (goto _label :!via `Open`))

(event `eCloseAddDescGate`
  ;[1 1 1] Additional Desc
  (goto _label :!via `Close`))

(event `evToggleAdditionalDescOff`
  ;[1 1 1] Toggle Off Additional Desc
  (`self.evCloseDesc1Gate`)
  (`self.eCloseAddDescGate`)
  (`self.evCounterOpen`)
  (`self.evQuitNoInspectClose`))

(event `evEmptyDescOpen`
  ;[1 1 1] Empty Desc
  (goto _label_4 :!via `Open`))

(event `self.Interact`
  (params (PlayerCharacter :type "/Game/Player/SP_PlayerCharacter Object Reference"))
  (set `self.Player Character` PlayerCharacter)
  (`|ExecutionSequence`
    (:`then_0`
      ;[1 1 1] Additional Desc
      (`|ExecutionSequence`
        (:`then_0`
          (if (`self.HasAdditionalDesc?`)
            (`/Engine/EditorBlueprintResources/StandardMacros.DoOnce` false
              (:`Completed`
                (`self.evCloseDesc1Gate`)
                (`self.evOpenAddDescGate`)
                (`self.evCounterClose`)
                (`self.evQuitNoInspectOpen`)))))
        (:`then_1`
          (`/Engine/EditorBlueprintResources/StandardMacros.Gate` true :!label _label
            (:`Exit`
              (`/Engine/EditorBlueprintResources/StandardMacros.DoOnce` false :!label _label_2
                (:`Completed`
                  (`|ExecutionSequence`
                    (:`then_0`
                      (if (`self.HasInspectView`)
                        (`self.fnStartInspectView`)))
                    (:`then_1`
                      (`self.fnDisableCharInput`)
                      (bind _returnvalue (`|CreateWidget` "/Game/UI/Interaction/W_PropDesc.W_PropDesc_C" null (`self.Additional Desc`)))
                      (bind _output_get (set `self.DescWidget Ref` _returnvalue))
                      (`UserWidget.AddToViewport` _output_get 0)
                      (`KismetSystemLibrary.Delay` 0.2)
                      (`GameplayStatics.SetGlobalTimeDilation` 0.0)
                      (`GameplayStatics.SetGamePaused` true)
                      (`GameplayStatics.SetGlobalTimeDilation` 1.0)
                      (if (`self.RepeatableDesc?`)
                        (goto _label_2 :!via `Reset`)
                        (else
                          (`self.fnInteractionOff`))))))))))))
    (:`then_1`
      (`/Engine/EditorBlueprintResources/StandardMacros.Gate` false :!label _label_3
        (:`Exit`
          (`|ExecutionSequence`
            (:`then_0`
              ;[1 1 1] Empty Desc
              (`/Engine/EditorBlueprintResources/StandardMacros.Gate` true :!label _label_4
                (:`Exit`
                  (`|ExecutionSequence`
                    (:`then_0`
                      (if (`self.HasInspectView`)
                        (`PlayerController.SetViewTargetWithBlend` (`GameplayStatics.GetPlayerController` 0) self 0.0 "VTBlend_Linear" 0.0 false)))
                    (:`then_1`
                      (`self.fnDisableCharInput`)
                      (bind _returnvalue_2 (`|CreateWidget` "/Game/UI/Interaction/W_PropDesc.W_PropDesc_C" null (`self.Empty Description`)))
                      (bind _output_get_2 (set `self.DescWidget Ref` _returnvalue_2))
                      (`UserWidget.AddToViewport` _output_get_2 0)
                      (`|ExecutionSequence`
                        (:`then_0`
                          (`KismetSystemLibrary.Delay` 0.2)
                          (`GameplayStatics.SetGlobalTimeDilation` 0.0)
                          (`GameplayStatics.SetGamePaused` true)
                          (`GameplayStatics.SetGlobalTimeDilation` 1.0))
                        (:`then_1`
                          (`/Engine/EditorBlueprintResources/StandardMacros.DoOnce` false
                            (:`Completed`
                              (`self.OnDescEnded`))))))))))
            (:`then_1`
              (`/Engine/EditorBlueprintResources/StandardMacros.Gate` false :!label _label_5
                (:`Exit`
                  ;[1 1 1] Desc 1
                  (if (`self.HasDesc1`)
                    (`|ExecutionSequence`
                      (:`then_0`
                        (if (`self.HasInspectView`)
                          (`PlayerController.SetViewTargetWithBlend` (`GameplayStatics.GetPlayerController` 0) self 0.0 "VTBlend_PreBlended" 0.0 false)))
                      (:`then_1`
                        (`self.fnDisableCharInput`)
                        (bind _returnvalue_3 (`|CreateWidget` "/Game/UI/Interaction/W_PropDesc.W_PropDesc_C" null (`self.Description1`)))
                        (bind _output_get_3 (set `self.DescWidget Ref` _returnvalue_3))
                        (`UserWidget.AddToViewport` _output_get_3 0)
                        (`|ExecutionSequence`
                          (:`then_0`
                            (`KismetSystemLibrary.Delay` 0.2)
                            (`GameplayStatics.SetGlobalTimeDilation` 0.0)
                            (`GameplayStatics.SetGamePaused` true)
                            (`GameplayStatics.SetGlobalTimeDilation` 1.0))
                          (:`then_1`
                            (`/Engine/EditorBlueprintResources/StandardMacros.DoOnce` false
                              (:`Completed`
                                (add `self.OnDescEnded` (`|CreateDelegate` :!event `evQuitNoInspectOpen`))))))))
                    (else
                      ;[1 1 1] No Desc - Gives Item
                      (if (`self.GivesQuestObject?`)
                        (`self.fnDisableCharInput`)
                        (`GameplayStatics.SetGamePaused` true)
                        (`self.evCounterClose`)
                        (`self.fnGiveQuestItem` (`self.Player Character`))
                        (if (`self.HasEmptyDesc?`)
                          (`self.evEmptyDescOpen`)
                          (`self.evDesc1Close`)
                          (`/Engine/EditorBlueprintResources/StandardMacros.DoOnce` false
                            (:`Completed`
                              (add `self.OnDescEnded` (`|CreateDelegate` :!event `evQuitNoInspectOpen`))
                              (`self.fnRemoveDescWidget`)))
                          (else
                            (`self.fnInteractionOff`)))
                        (else
                          (`self.fnInteractionOff`))))))))))))))

(event `evDesc1Close`
  (goto _label_5 :!via `Close`))

(event `evOpenDesc1Gate`
  (goto _label_3 :!via `Open`))

(event `evCloseDesc1Gate`
  (goto _label_3 :!via `Close`))

(event `evQuitNoInspectOpen`
  ;[1 1 1] Counter Loop
  (goto _label_6 :!via `Open`))

(event `evQuitNoInspectClose`
  ;[1 1 1] Counter Loop
  (goto _label_6 :!via `Close`))

(event `EnhancedInput|/Game/Player/Input/IA_Interact`
  (params (ActionValue :type Boolean) (ElapsedSeconds :type "Float (double-precision)") (TriggeredSeconds :type "Float (double-precision)") (InputAction :type "InputAction Object Reference" :default "/Game/Player/Input/IA_Interact.IA_Interact"))
  ;[1 1 1] Counter Loop
  (:`Triggered`
    (`|ExecutionSequence`
      (:`then_0`
        (`/Engine/EditorBlueprintResources/StandardMacros.Gate` true :!label _label_6
          (:`Exit`
            (`self.fnQuitWithoutInspect`))))
      (:`then_1`
        (`/Engine/EditorBlueprintResources/StandardMacros.Gate` false :!label _label_7
          (:`Exit`
            (`|ExecutionSequence`
              (:`then_0`
                (if (< (`self.DescCounter`) 3)
                  (`/Engine/EditorBlueprintResources/StandardMacros.IncrementInt` (`self.DescCounter`))))
              (:`then_1`
                (if (== (`self.DescCounter`) 1)
                  ;[1 1 1] Has Desc2 ?
                  (if (`self.HasDesc2`)
                    (`self.fnChangeText` (`self.Description 2`))
                    (elif (`self.GivesQuestObject?`)
                      (`self.fnGiveQuestItem` (`self.Player Character`))
                      (if (`self.HasEmptyDesc?`)
                        (`self.evEmptyDescOpen`)
                        (`self.evDesc1Close`)
                        (elif (`self.RepeatableDesc?`)
                          (set `self.DescCounter` 0)
                          (else
                            (`self.fnInteractionOff`))))
                      ;[1 1 1] Leave Descriptions
                      (`self.fnRemoveDescWidget` :!label _label_8)
                      (if (`self.IsDestroyedAfter?`)
                        (`self.K2_DestroyActor`))
                      (else
                        (if (`self.HasEmptyDesc?`)
                          (`self.evEmptyDescOpen`)
                          (`self.evDesc1Close`)
                          (`self.evCounterClose` :!label _label_9)
                          (elif (`self.RepeatableDesc?`)
                            (goto _label_9)
                            (else
                              (`self.fnInteractionOff`))))
                        (`self.fnQuitWithoutInspect`))))
                  (else
                    ;[1 1 1] Has Desc3 ?
                    (if (== (`self.DescCounter`) 2)
                      (if (`self.HasDesc3`)
                        (`self.fnChangeText` (`self.Description 3`))
                        (elif (`self.GivesQuestObject?`)
                          (`self.fnGiveQuestItem` (`self.Player Character`))
                          (if (`self.HasEmptyDesc?`)
                            (`self.evEmptyDescOpen`)
                            (`self.evDesc1Close`)
                            (goto _label_8)
                            (elif (`self.RepeatableDesc?`)
                              (set `self.DescCounter` 0)
                              (goto _label_8)
                              (else
                                (`self.fnInteractionOff`)
                                (goto _label_8))))
                          (else
                            (if (`self.HasEmptyDesc?`)
                              (`self.evEmptyDescOpen`)
                              (`self.evDesc1Close`)
                              (elif (`self.RepeatableDesc?`)
                                (set `self.DescCounter` 0)
                                (else
                                  (`self.fnInteractionOff`))))
                            (`self.fnQuitWithoutInspect`))))
                      (else
                        ;[1 1 1] Final after Desc3
                        (if (== (`self.DescCounter`) 3)
                          (if (`self.GivesQuestObject?`)
                            (`self.fnGiveQuestItem` (`self.Player Character`))
                            (if (`self.HasEmptyDesc?`)
                              (`self.evEmptyDescOpen`)
                              (`self.evDesc1Close`)
                              (goto _label_8)
                              (elif (`self.RepeatableDesc?`)
                                (set `self.DescCounter` 0)
                                (goto _label_8)
                                (else
                                  (`self.fnInteractionOff`)
                                  (goto _label_8))))
                            (else
                              (if (`self.HasEmptyDesc?`)
                                (`self.evEmptyDescOpen`)
                                (`self.evDesc1Close`)
                                (elif (`self.RepeatableDesc?`)
                                  (set `self.DescCounter` 0)
                                  (else
                                    (`self.fnInteractionOff`))))
                              (`self.fnQuitWithoutInspect`)))
                          (else
                            (`KismetSystemLibrary.PrintString` "ERROR: Counter more than 3")))))))))))))))

(event `evCounterOpen`
  ;[1 1 1] Counter Loop
  (goto _label_7 :!via `Open`))

(event `evCounterClose`
  ;[1 1 1] Counter Loop
  (goto _label_7 :!via `Close`))

(event `self.ShowHUD`
  ;[1 1 1] Show Hint Logic
  (if (`PrimitiveComponent.IsOverlappingActor` (`self.innerSphereCollision`) (`GameplayStatics.GetPlayerCharacter` 0))
    (`SceneComponent.SetVisibility` (`self.innerInteractionIcon`) true false)
    (if (`self.IsMainGoal?`)
      (`SceneComponent.SetVisibility` (`self.outerInteractionIcon`) false false))
    (else
      (`SceneComponent.SetVisibility` (`self.innerInteractionIcon`) false false :!label _label_10)
      (if (`self.IsMainGoal?`)
        (`SceneComponent.SetVisibility` (`self.outerInteractionIcon`) true false)))))

(event `self.HideHUD`
  ;[1 1 1] Show Hint Logic
  (if (`PrimitiveComponent.IsOverlappingActor` (`self.innerSphereCollision`) (`GameplayStatics.GetPlayerCharacter` 0))
    (goto _label_10)))

(event `self.outerSphereCollision.OnComponentBeginOverlap`
  (params (OverlappedComponent :type "PrimitiveComponent Object Reference") (OtherActor :type "Actor Object Reference") (OtherComp :type "PrimitiveComponent Object Reference") (OtherBodyIndex :type Integer) (bFromSweep :type Boolean) (SweepResult :type "HitResult Structure (by ref)"))
  ;[1 1 1] Show Hint Logic
  (if (and (== OtherActor (`GameplayStatics.GetPlayerCharacter` 0)) (`self.IsMainGoal?`))
    (`SceneComponent.SetVisibility` (`self.outerInteractionIcon`) true false)))

(event `self.outerSphereCollision.OnComponentEndOverlap`
  (params (OverlappedComponent :type "PrimitiveComponent Object Reference") (OtherActor :type "Actor Object Reference") (OtherComp :type "PrimitiveComponent Object Reference") (OtherBodyIndex :type Integer))
  ;[1 1 1] Show Hint Logic
  (if (and (`self.IsMainGoal?`) (== (`GameplayStatics.GetPlayerCharacter` 0) OtherActor))
    (`SceneComponent.SetVisibility` (`self.outerInteractionIcon`) false false)))

(fn `fnChangeText`
  (params (`Text Line` :type Text))
  (`TextBlock.SetText` (`/Game/UI/Interaction/W_PropDesc.TXT_Description` (`self.DescWidget Ref`)) `Text Line`))

(fn `fnDisableCharInput`
  (bind _returnvalue (`GameplayStatics.GetPlayerController` 0))
  (`self.DisableInput` (`GameplayStatics.GetPlayerCharacter` 0) _returnvalue)
  (`self.EnableInput` _returnvalue))

(fn `fnEnableCharInput`
  (bind _returnvalue (`GameplayStatics.GetPlayerController` 0))
  (`self.DisableInput` _returnvalue)
  (`self.EnableInput` (`GameplayStatics.GetPlayerCharacter` 0) _returnvalue))

(fn `fnGiveQuestItem`
  (params (`Player Character` :type "/Game/Player/SP_PlayerCharacter Object Reference"))
  (bind _ac_inventory (`/Game/Player/SP_PlayerCharacter.AC_Inventory` `Player Character`))
  (bind (_quest_object_datatable _quest_object_rowname) (break `DataTableRowHandle` (`self.Quest Object`)))
  (`|ExecutionSequence`
    (:`then_0`
      (if (`self.HasInspectView`)
        (`PlayerController.SetViewTargetWithBlend` (`GameplayStatics.GetPlayerController` 0) (`self.NextCamera`) 0.0 "VTBlend_Linear" 0.0 false)))
    (:`then_1`
      (bind _returnvalue (`|SpawnActorFromClass` "/Game/Blueprints/Actors/BP_InspectItem.BP_InspectItem_C" (`KismetMathLibrary.MakeTransform` (100000000.0 0.0 0.0)) "Undefined" "MultiplyWithRoot" null null))
      (`/Engine/EditorBlueprintResources/StandardMacros.IsValid` _ac_inventory
        (:`Is Valid`
          (bind _returnvalue_2 (`|GetDataTableRow` _quest_object_datatable _quest_object_rowname)
            (:`then`
              (bind (_name _description _mesh _itemactor _thumbnail _stacksize) (break `/Game/Blueprints/Structs/STR_QuestItems` _returnvalue_2))
              (bind _success (`/Game/Blueprints/ActorComponents/AC_Inventory.fnAddToInventory` _ac_inventory _quest_object_rowname _stacksize))
              (if _success
                (set `self.GivesQuestObject?` false)
                (message `/Game/Blueprints/BPInterfaces/BPi_Interact.Inspect` _returnvalue `Player Character` _mesh _name _description null true true)
                (if (`self.IsMainGoal?`)
                  (`self.dspCheckInteracted`))
                (else
                  (`KismetSystemLibrary.PrintString` "Can't add Item")
                  (`self.fnQuitWithoutInspect`))))))))))

(fn `fnInteractionOff`
  (`PrimitiveComponent.SetCollisionResponseToChannel` (`self.StaticMesh`) "ECC_GameTraceChannel1" "ECR_Ignore")
  (`PrimitiveComponent.SetCollisionEnabled` (`self.innerSphereCollision`) "NoCollision")
  (`PrimitiveComponent.SetCollisionEnabled` (`self.outerSphereCollision`) "NoCollision")
  (`SceneComponent.SetVisibility` (`self.innerInteractionIcon`) false false)
  (`SceneComponent.SetVisibility` (`self.outerInteractionIcon`) false false))

(fn `fnInteractionOn`
  (`PrimitiveComponent.SetCollisionResponseToChannel` (`self.StaticMesh`) "ECC_GameTraceChannel1" "ECR_Block")
  (`PrimitiveComponent.SetCollisionEnabled` (`self.innerSphereCollision`) "QueryOnly")
  (`PrimitiveComponent.SetCollisionEnabled` (`self.outerSphereCollision`) "QueryOnly"))

(fn `fnQuitWithoutInspect`
  (`self.fnEnableCharInput`)
  (`self.fnRemoveDescWidget`)
  (`GameplayStatics.SetGamePaused` false)
  (if (`self.HasInspectView`)
    (`PlayerController.SetViewTargetWithBlend` (`GameplayStatics.GetPlayerController` 0) (`self.NextCamera`) 0.0 "VTBlend_Linear" 0.0 false)
    (if (`self.RepeatableDesc?`)
      (`self.fnInteractionOn`))))

(fn `fnRemoveDescWidget`
  (bind _descwidget_ref (`self.DescWidget Ref`))
  (`/Engine/EditorBlueprintResources/StandardMacros.IsValid` _descwidget_ref
    (:`Is Valid`
      (`Widget.RemoveFromParent` _descwidget_ref))
    (:`Is Not Valid`
      (`KismetSystemLibrary.PrintString` "DescWidget doesn't exist"))))

(fn `fnStartInspectView`
  (`PlayerController.SetViewTargetWithBlend` (`GameplayStatics.GetPlayerController` 0) self 0.0 "VTBlend_Linear" 0.0 false)
  (`self.fnInteractionOff`))

(fn `IsExaminable`
  (returns (IsExaminable :type Boolean))
  (return false))

(fn `IsInteractable`
  (returns (IsInteractable :type Boolean))
  (return true))

(fn `IsPickable`
  (returns (IsPickable :type Boolean))
  (return false))

(fn `UserConstructionScript`
  (bind _staticmesh (`self.StaticMesh`))
  (bind _inspectcamera (`self.InspectCamera`))
  (bind (_datatable _rowname) (break `DataTableRowHandle` (`self.Item ID`)))
  (`|ExecutionSequence`
    (:`then_0`
      (bind _returnvalue (`|GetDataTableRow` _datatable _rowname)
        (:`then`
          (`|ExecutionSequence`
            (:`then_0`
              (bind (_mesh _questobject _description1 _description2 _description3 _emptydescription _additionaldesc) (break `/Game/Blueprints/Structs/STR_InterProps` _returnvalue))
              (bind _output_get (set `self.Mesh` _mesh))
              (`StaticMeshComponent.SetStaticMesh` _staticmesh _output_get)
              (if (`self.HiddenMesh`)
                (`PrimitiveComponent.SetCollisionResponseToAllChannels` _staticmesh "ECR_Ignore")
                (`PrimitiveComponent.SetCollisionResponseToChannel` _staticmesh "ECC_GameTraceChannel1" "ECR_Block")))
            (:`then_1`
              (set `self.Description1` _description1))
            (:`then_2`
              (set `self.Description 2` _description2))
            (:`then_3`
              (set `self.Description 3` _description3))
            (:`then_4`
              (set `self.Quest Object` _questobject))
            (:`then_5`
              (set `self.Empty Description` _emptydescription))
            (:`then_6`
              (set `self.Additional Desc` _additionaldesc))))))
    (:`then_1`
      (`SphereComponent.SetSphereRadius` (`self.outerSphereCollision`) (`self.OuterInterSphereRadius`) true)
      (`SphereComponent.SetSphereRadius` (`self.innerSphereCollision`) (`self.InnerInterSphereRadius`) true)
      (`SceneComponent.K2_SetRelativeLocation` (`self.outerInteractionIcon`) (`self.IconLocation`) false false)
      (`SceneComponent.K2_SetRelativeLocation` (`self.innerInteractionIcon`) (`self.IconLocation`) false false))
    (:`then_2`
      ;[1 1 1] Debuggin Mode
      (if (`self.Debugging?`)
        (`SceneComponent.SetVisibility` (`self.outerSphereCollision`) true false)
        (`SceneComponent.SetVisibility` (`self.innerSphereCollision`) true false)
        (`SceneComponent.SetVisibility` (`self.outerInteractionIcon`) true false)
        (`SceneComponent.SetVisibility` (`self.innerInteractionIcon`) true false)
        (`|ExecutionSequence`
          (:`then_0`
            (if (`self.HasInspectView`)
              (`SceneComponent.SetWorldScale3D` (`self.InspectCamera`) (0.5 0.5 0.5))
              (else
                (`SceneComponent.SetWorldScale3D` (`self.InspectCamera`) (0.0 0.0 0.0) :!label _label))))
          (:`then_1`
            (if (`self.HiddenMesh`)
              (`SceneComponent.SetVisibility` (`self.StaticMesh`) true false)
              (else
                (`SceneComponent.SetVisibility` (`self.StaticMesh`) false false :!label _label_2)))))
        (else
          (`SceneComponent.SetVisibility` (`self.outerSphereCollision`) false false)
          (`SceneComponent.SetVisibility` (`self.innerSphereCollision`) false false)
          (`SceneComponent.SetVisibility` (`self.outerInteractionIcon`) false false)
          (`SceneComponent.SetVisibility` (`self.innerInteractionIcon`) false false)
          (`|ExecutionSequence`
            (:`then_0`
              (if (`self.HasInspectView`)
                (goto _label)
                (else
                  (goto _label))))
            (:`then_1`
              (if (`self.HiddenMesh`)
                (goto _label_2)))))))
    (:`then_3`
      (if (`self.HasInspectView`)
        (`ActorComponent.SetAutoActivate` (`self.InspectCamera`) true)
        (set `self.Inspect Camera ref` (`self.InspectCamera`))
        (`SceneComponent.K2_SetRelativeLocation` (`self.InspectCamera`) (`self.Location`) false false)
        (`SceneComponent.K2_SetWorldRotation` (`self.InspectCamera`) (`self.Rotation`) false false)
        (else
          (`ActorComponent.SetAutoActivate` _inspectcamera false)
          (`SceneComponent.SetVisibility` _inspectcamera false false)
          (set `CameraComponent.bLockToHmd` false _inspectcamera))))))