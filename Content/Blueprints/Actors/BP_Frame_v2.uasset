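; Rotatable frame actor that turns its pivot in yaw when its clockwise or counter-clockwise child-actor buttons are interacted with.
; BeginPlay binds two buttons per direction to rotation events, each playing a timeline whose alpha is added to the starting yaw.
; A shared Recharging flag blocks overlapping turns, and per-direction DoOnce gates reset only when their own timeline finishes.
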(event `self.ReceiveBeginPlay`
  (add `/Game/Blueprints/Actors/BP_ButtonNonClockwise.Interacted NonClockwise` (`|MakeArray` (cast `/Game/Blueprints/Actors/BP_ButtonNonClockwise` (`ChildActorComponent.ChildActor` (`self.NonClockwiseButton2`)) :!pure true) (cast `/Game/Blueprints/Actors/BP_ButtonNonClockwise` (`ChildActorComponent.ChildActor` (`self.NonClockwiseButton1`)) :!pure true)) (delegate `evRotateNonClockwise`))
  (add `/Game/Blueprints/Actors/BP_ButtonClockwise.Interacted Clockwise` (`|MakeArray` (cast `/Game/Blueprints/Actors/BP_ButtonClockwise` (`ChildActorComponent.ChildActor` (`self.ClockwiseButton2`)) :!pure true) (cast `/Game/Blueprints/Actors/BP_ButtonClockwise` (`ChildActorComponent.ChildActor` (`self.ClockwiseButton1`)) :!pure true)) (delegate `evRotateClockwise`)))

(event `evRotateClockwise`
  (bind _framepivot (`self.FramePivot`))
  (bind (_relativerotation_roll _relativerotation_pitch _relativerotation_yaw) (`KismetMathLibrary.BreakRotator` (`SceneComponent.RelativeRotation` (`self.FramePivot`))))
  (bind (_relativerotation_roll_2 _relativerotation_pitch_2) (`KismetMathLibrary.BreakRotator` (`SceneComponent.RelativeRotation` _framepivot)))
  (`/Engine/EditorBlueprintResources/StandardMacros.DoOnce` false :!label _label
    (:`Completed`
      (if (not (`self.Recharging`))
        (set `self.Start Rotation` _relativerotation_yaw)
        (set `self.Recharging` true)
        (bind (_direction _alpha) (`Timeline|Clockwise Rotation` :!via `PlayFromStart`)
          (:`Update`
            (`SceneComponent.K2_SetRelativeRotation` _framepivot (`KismetMathLibrary.MakeRotator` _relativerotation_roll_2 _relativerotation_pitch_2 (+ (`self.Start Rotation`) _alpha)) false false))
          (:`Finished`
            (set `self.Recharging` false)
            (goto _label :!via `Reset`)))))))

(event `evRotateNonClockwise`
  (bind _framepivot (`self.FramePivot`))
  (bind (_relativerotation_roll _relativerotation_pitch) (`KismetMathLibrary.BreakRotator` (`SceneComponent.RelativeRotation` _framepivot)))
  (bind (_relativerotation_roll_2 _relativerotation_pitch_2 _relativerotation_yaw) (`KismetMathLibrary.BreakRotator` (`SceneComponent.RelativeRotation` (`self.FramePivot`))))
  (`/Engine/EditorBlueprintResources/StandardMacros.DoOnce` false :!label _label_2
    (:`Completed`
      (if (not (`self.Recharging`))
        (set `self.Start Rotation` _relativerotation_yaw)
        (set `self.Recharging` true)
        (bind (_direction _alpha) (`Timeline|Non-Clockwise Rotation` :!via `PlayFromStart`)
          (:`Update`
            (`SceneComponent.K2_SetRelativeRotation` _framepivot (`KismetMathLibrary.MakeRotator` _relativerotation_roll _relativerotation_pitch (+ (`self.Start Rotation`) _alpha)) false false))
          (:`Finished`
            (set `self.Recharging` false)
            (goto _label_2 :!via `Reset`)))))))

(fn `UserConstructionScript`)