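; BP_PillarButton is an interactable, non-examinable button actor.
; Interact fires the IsActivated event dispatcher to notify listeners, then plays the MoveDown timeline.
; The timeline's Alpha track sets the actor's Z location directly as an absolute world height, keeping X and Y unchanged.
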(event `/Game/Blueprints/BPInterfaces/BPi_Interact.Interact`
  (params (PlayerCharacter :type "/Game/Characters/Player/SP_PlayerCharacter Object Reference"))
  (bind (_returnvalue_x _returnvalue_y) (`KismetMathLibrary.BreakVector` (`self.K2_GetActorLocation` self)))
  (`self.IsActivated?`)
  (bind (_direction _alpha) (`Timeline|Move Down`)
    (:`Update`
      (`self.K2_SetActorLocation` self (`KismetMathLibrary.MakeVector` _returnvalue_x _returnvalue_y _alpha) false false))))

(fn `IsExaminable`
  (returns (IsExaminable :type Boolean))
  (return false))

(fn `IsInteractable`
  (returns (IsInteractable :type Boolean))
  (return true))

(fn `UserConstructionScript`
  (`parent.UserConstructionScript`))