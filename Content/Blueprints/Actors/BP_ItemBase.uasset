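; Base item actor that handles using an item on a target implementing BPI_Interactable.
; Useon looks up the ItemID in DT_ItemUsageRule; a matching target class receives DoOpenDoor, then OnItemUsedSuccessfully fires if the rule or item is consumable.
; A missing row or class mismatch falls back to passing the item through OnUseItem on the target.
; The consume event is an empty stub, and the inventory removal logic is disconnected.
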(event `/Game/Blueprints/Interfaces/BPI_UsableItem.UseOn`
  (params (Target :type "Actor Object Reference"))
  (`/Engine/EditorBlueprintResources/StandardMacros.IsValid` Target
    (:`Is Valid`
      (bind _returnvalue (`self.CanBeUsedOn` Target))
      (if _returnvalue
        (bind _returnvalue_2 (`|GetDataTableRow` "/Game/Data/DTs/DT_ItemUsageRule.DT_ItemUsageRule" (`self.ItemID`))
          (:`then`
            (set `self.bFound?` true)
            (bind _output_get (set `self.UsageRow` _returnvalue_2))
            (if (`KismetMathLibrary.ClassIsChildOf` (`GameplayStatics.GetObjectClass` Target) (`.TargetClass_8_28E75C124989E22622A182AAE578A3CE` (break `/Game/Data/Structs/STR_ItemUsageRule` _output_get)))
              (message `/Game/Blueprints/BPInterfaces/BPI_ActionReciever.Do_OpenDoor` Target)
              (if (or (`.ConsumeOnSuccess_12_208E10DA41DA61EEB4A167A183A59A0B` (break `/Game/Data/Structs/STR_ItemUsageRule` (`self.UsageRow`))) (`self.bConsumable`))
                (message `/Game/Blueprints/Interfaces/BPI_UsableItem.OnItemUsedSuccessfully` self (`self.ItemID`)))
              (else
                (message `/Game/Blueprints/Interfaces/BPI_Interactable.OnUseItem` Target self))))
          (:`RowNotFound`
            (set `self.bFound?` false)
            (set `self.UsageRow` (struct))
            (message `/Game/Blueprints/Interfaces/BPI_Interactable.OnUseItem` Target self)))))))

(event `evConsumeItem`)

(fn `CanBeUsedOn`
  (params (Target :type "Actor Object Reference"))
  (returns (ReturnValue :type Boolean))
  (return (`KismetSystemLibrary.DoesImplementInterface` Target "/Game/Blueprints/Interfaces/BPI_Interactable.BPI_Interactable_C")))