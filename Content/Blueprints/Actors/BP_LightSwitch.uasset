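; BP_LightSwitch is an interactable switch actor that toggles a linked light on and off.
; Its Interact event checks IsLightOn on the BPLight reference and calls that light's turn-off or turn-on function.
; It reports itself as interactable but not examinable, and returns empty look-at text.
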(event `/Game/Blueprints/Interaction/BPi_Interact.Interact`
  (params (PlayerCharacter :type "/Game/Characters/Player/SP_PlayerCharacter Object Reference"))
  (bind _bp_light (`self.BP Light`))
  (if (`/Game/Blueprints/Actors/BP_Light.IsLightOn?` _bp_light)
    (`/Game/Blueprints/Actors/BP_Light.fnTurnOffLight` _bp_light)
    (else
      (`/Game/Blueprints/Actors/BP_Light.fnTurnOnLight` _bp_light))))

(fn `IsExaminable`
  (returns (IsExaminable :type Boolean))
  (return false))

(fn `IsInteractable`
  (returns (IsInteractable :type Boolean))
  (return true))

(fn `LookAt`
  (returns (Messege :type Text))
  (return ""))

(fn `UserConstructionScript`)