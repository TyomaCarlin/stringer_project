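; BP_Doors is an interactable, non-examinable door actor that can optionally require a key.
; Interact toggles the door by playing or reversing the OpenDoor timeline, which swings the Pivot component a quarter turn in yaw.
; When a key is required, PickUpKey must have set HasKey, otherwise a "Get the Key" message prints.
; Each opening also fires the IsDoorOpened dispatcher.
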(event `/Game/Blueprints/BPInterfaces/BPi_Interact.Interact`
  (params (PlayerCharacter :type "/Game/Characters/Player/SP_PlayerCharacter Object Reference"))
  (if (`self.KeyRequired?`)
    (if (`self.HasKey`)
      (if (`self.IsClosed`) :!label _label
        (set `self.IsClosed` false)
        (`self.IsDoorOpened?`)
        (bind (_direction _alpha) (`Timeline|Open Door` :!label _label_2)
          (:`Update`
            (`SceneComponent.K2_SetRelativeRotation` (`self.Pivot`) (`KismetMathLibrary.MakeRotator` 0.0 0.0 (`KismetMathLibrary.Lerp` 0.0 -90.0 _alpha)) false false)))
        (else
          (set `self.IsClosed` true)
          (goto _label_2 :!via `Reverse`)))
      (else
        (`KismetSystemLibrary.PrintString` "Get the Key")))
    (else
      (goto _label))))

(event `/Game/Blueprints/BPInterfaces/BPi_Keys.PickUpKey`
  (set `self.HasKey` true))

(fn `IsExaminable`
  (returns (IsExaminable :type Boolean))
  (return false))

(fn `IsInteractable`
  (returns (IsInteractable :type Boolean))
  (return true))

(fn `UserConstructionScript`
  (`parent.UserConstructionScript`))