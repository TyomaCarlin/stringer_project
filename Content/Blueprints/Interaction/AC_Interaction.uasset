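; Actor component on the player character that detects interactable objects in view and handles the interact input.
; Each tick, a box trace runs forward from the camera, caching hit actors that pass the interactable message check and toggling a "Press E" prompt in a widget created on BeginPlay.
; IA_Interact sends the cached object either an examine or an interact message, setting IsExamining accordingly.
; LookAt is a stub returning an empty value.
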(event `self.ReceiveBeginPlay`
  (bind _returnvalue (`|CreateWidget` "/Game/UI/W_Message.W_Message_C"))
  (bind _output_get (set `self.Widget Message` _returnvalue))
  (`UserWidget.AddToViewport` _output_get 0))

(event `self.ReceiveTick`
  (params (DeltaSeconds :type "Float (single-precision)"))
  (bind _camera (`/Game/Characters/Player/SP_PlayerCharacter.Camera` (cast `/Game/Characters/Player/SP_PlayerCharacter` (`self.GetOwner`) :!pure true)))
  (bind _returnvalue (`SceneComponent.K2_GetComponentLocation` _camera))
  (bind (_outhit _returnvalue_2) (`KismetSystemLibrary.BoxTraceSingle` _returnvalue (+ _returnvalue (* (`KismetMathLibrary.GetForwardVector` (`SceneComponent.K2_GetComponentRotation` _camera)) (`self.InterDistance`))) (`self.Trace Size`) (struct) "TraceTypeQuery3" false (`|MakeArray` (`self.GetOwner`)) "None" true (struct :`R` 1.0 :`A` 1.0) (struct :`G` 1.0 :`A` 1.0) 1.0))
  (if _returnvalue_2
    (bind (_bblockinghit _binitialoverlap _time _distance _location _impactpoint _normal _impactnormal _physmat _hitactor) (`GameplayStatics.BreakHitResult` _outhit))
    (bind _isinteractable (message `/Game/Blueprints/BPInterfaces/BPi_Interact.IsInteractable` _hitactor))
    (if _isinteractable
      (set `self.Hit Object` _hitactor)
      (`/Game/UI/W_Message.ShowMessage` (`self.Widget Message`) "Press E")
      (else
        (set `self.Hit Object` null :!label _label)
        (`/Game/UI/W_Message.ShowMessage` (`self.Widget Message`) "")))
    (else
      (goto _label))))

(event `EnhancedInput|/Game/Input/IA_Interact`
  (params (ActionValue :type Boolean) (ElapsedSeconds :type "Float (double-precision)") (TriggeredSeconds :type "Float (double-precision)") (InputAction :type "InputAction Object Reference" :default "/Game/Input/IA_Interact.IA_Interact"))
  (bind _hit_object (`self.Hit Object`))
  (:`Triggered`
    (bind _isexaminable (message `/Game/Blueprints/BPInterfaces/BPi_Interact.IsExaminable` (`self.Hit Object`)))
    (if _isexaminable
      (message `/Game/Blueprints/BPInterfaces/BPi_Interact.Examine` _hit_object)
      (set `self.IsExamining` true)
      (else
        (message `/Game/Blueprints/BPInterfaces/BPi_Interact.Interact` _hit_object (cast `/Game/Characters/Player/SP_PlayerCharacter` (`self.GetOwner`) :!pure true))
        (set `self.IsExamining` false)))))

(fn `LookAt`
  (params (NewParam :type Boolean))
  (returns (Messege :type Text))
  (return ""))