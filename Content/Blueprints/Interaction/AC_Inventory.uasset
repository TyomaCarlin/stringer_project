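; Inventory component holding a fixed-size array of item slots, with add, remove, consume, quantity query and slot transfer functions.
; Adding works one unit at a time, topping up stacks to the DT_InventorySlots limit before filling empty slots, and returns any remainder.
; Changes broadcast OnInventoryUpdated, directly or via MC_Update, except low-level stack helpers.
; Transfer swaps differing items only for negative destination indices; autosave is an unbound stub, and key 1 prints contents.
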(event `MC_Update`
  (`self.OnInventoryUpdated`))

(event `self.ReceiveBeginPlay`
  (`KismetArrayLibrary.Array_Resize` (`self.Contents`) (`self.InventorySize`)))

(event `AutoSaveInventory`)

(event `Key|One`
  (params (Key :type "Key Structure"))
  (:`Pressed`
    (`self.DEBUG_PrintContents`)))

(fn `DEBUG_PrintContents`
  (for (_array_element _array_index) (`self.Contents`)
    (bind (_itemid _quantity) (break `/Game/Blueprints/Interaction/STR_InventorySlots` _array_element))
    (`KismetSystemLibrary.PrintString` (`KismetStringLibrary.Concat_StrStr` (`KismetStringLibrary.Conv_IntToString` _array_index) ":" (`KismetStringLibrary.Conv_NameToString` _itemid) "=" (`KismetStringLibrary.Conv_IntToString` _quantity)))))

(fn `fnAddToInventory`
  (params (ItemID :type Name) (Quantity :type Integer))
  (returns (Success :type Boolean) (QuantityRemained :type Integer))
  (locals (Local_QuantityRemained :type Integer) (Local_HasFailed :type Boolean))
  (set `local.Local_QuantityRemained` Quantity)
  (while (and (> (`local.Local_QuantityRemained`) 0) (not (`local.Local_HasFailed`)))
    (bind (_index _slotfound) (`self.fnFindSuitableSlot` ItemID))
    (if _slotfound
      (`self.fnAddToStack` _index 1)
      (`/Engine/EditorBlueprintResources/StandardMacros.DecrementInt` (`local.Local_QuantityRemained`))
      (elif (`self.fnAnyEmptySlotsAvailable`)
        (bind _success (`self.fnCreateNewStack` (`local.ItemID`) 1))
        (if _success
          (`/Engine/EditorBlueprintResources/StandardMacros.DecrementInt` (`local.Local_QuantityRemained`))
          (else
            (set `local.Local_HasFailed` true)))
        (else
          (set `local.Local_HasFailed` true)))))
  (`self.OnInventoryUpdated`)
  (return (not (`local.Local_HasFailed`)) (`local.Local_QuantityRemained`)))

(fn `fnAddToStack`
  (params (Index :type Integer) (Quantity :type Integer))
  (bind _contents (`self.Contents`))
  (bind (_output_itemid _output_quantity) (break `/Game/Blueprints/Interaction/STR_InventorySlots` (`|GetArrayItem` _contents Index)))
  (`KismetArrayLibrary.Array_Set` _contents Index (make `/Game/Blueprints/Interaction/STR_InventorySlots` _output_itemid (+ _output_quantity Quantity))))

(fn `fnAnyEmptySlotsAvailable`
  (returns (HasEmptySlot :type Boolean) (EmptyIndex :type Integer))
  (for (_array_element _array_index) (`self.Contents`)
    (if (== (`.Quantity_5_8115720D48DA2592682C9D9C8ACA4122` (break `/Game/Blueprints/Interaction/STR_InventorySlots` _array_element)) 0)
      (return true _array_index)))
  (return false -1))

(fn `fnConsumeItem`
  (params (Index :type Integer))
  (locals (`Local ItemID` :type Name) (`Local Quantity` :type Integer))
  (bind (_output_itemid _output_quantity) (break `/Game/Blueprints/Interaction/STR_InventorySlots` (`|GetArrayItem` (`self.Contents`) Index)))
  (set `local.Local ItemID` _output_itemid)
  (set `local.Local Quantity` _output_quantity)
  (`|ExecutionSequence`
    (:`then_0`
      (`self.fnRemoveFromInventory` (`local.Index`)))
    (:`then_1`
      (`self.MC_Update`))))

(fn `fnCreateNewStack`
  (params (ItemID :type Name) (Quantity :type Integer))
  (returns (Success :type Boolean))
  (bind (_hasemptyslot _emptyindex) (`self.fnAnyEmptySlotsAvailable`))
  (if _hasemptyslot
    (`KismetArrayLibrary.Array_Set` (`self.Contents`) _emptyindex (make `/Game/Blueprints/Interaction/STR_InventorySlots` ItemID Quantity))
    (return true)
    (else
      (return false))))

(fn `fnFindSuitableSlot`
  (params (ItemID :type Name))
  (returns (Index :type Integer) (SlotFound :type Boolean))
  (for (_array_element _array_index) (`self.Contents`)
    (bind (_itemid _quantity) (break `/Game/Blueprints/Interaction/STR_InventorySlots` _array_element))
    (if (== _itemid ItemID)
      (if (< _quantity (`self.fnGetMaxStackSize` ItemID))
        (return _array_index true))))
  (return -1 false))

(fn `fnGetMaxStackSize`
  (params (ItemID :type Name))
  (returns (StackSize :type Integer))
  (bind _returnvalue (`|GetDataTableRow` "/Game/Blueprints/Interaction/DT_InventorySlots.DT_InventorySlots" ItemID)
    (:`then`
      (return (`.Quantity_5_8115720D48DA2592682C9D9C8ACA4122` (break `/Game/Blueprints/Interaction/STR_InventorySlots` _returnvalue))))
    (:`RowNotFound`
      (return -1))))

(fn `fnQueryInventory`
  (params (RequiredItemID :type Name) (RequiredQuantity :type Integer :default 1))
  (returns (Success :type Boolean) (OutQuantity :type Integer))
  (locals (RunningTotal :type Integer))
  (for _array_element (`self.Contents`)
    (bind (_itemid _quantity) (break `/Game/Blueprints/Interaction/STR_InventorySlots` _array_element))
    (if (== _itemid (`local.RequiredItemID`))
      (set `local.RunningTotal` (+ _quantity (`local.RunningTotal`)))))
  (return (>= (`local.RunningTotal`) (`local.RequiredQuantity`)) (`local.RunningTotal`)))

(fn `fnRemoveFromInventory`
  (params (Index :type Integer) (RemoveWholeStack :type Boolean))
  (locals (LocalItem :type Name) (LocalQuantity :type Integer))
  (bind (_output_itemid _output_quantity) (break `/Game/Blueprints/Interaction/STR_InventorySlots` (`|GetArrayItem` (`self.Contents`) Index)))
  (bind _output (`|GetArrayItem` (`self.Contents`) (`self.Index`)))
  (set `local.LocalItem` _output_itemid)
  (set `local.LocalQuantity` _output_quantity)
  (`|ExecutionSequence`
    (:`then_0`
      (if (or (`local.RemoveWholeStack`) (== (`local.LocalQuantity`) 1))
        (`KismetArrayLibrary.Array_Set` (`self.Contents`) (`local.Index`))
        (else
          (setmembers `/Game/Blueprints/Interaction/STR_InventorySlots` :`StructRef` _output :`Quantity` (- (`.Quantity_5_8115720D48DA2592682C9D9C8ACA4122` (break `/Game/Blueprints/Interaction/STR_InventorySlots` _output)) 1)))))
    (:`then_1`
      (`self.MC_Update`))))

(fn `fnTransferSlots`
  (params (`Source Index` :type Integer) (`Source Inventory` :type "/Game/Blueprints/Interaction/AC_Inventory Object Reference") (`Destination Index` :type Integer))
  (locals (LocalSlotContent :type " Structure") (LocalSlotContent :type Boolean) (LocalSlotArray :type "/Game/Blueprints/Interaction/STR_InventorySlots Structure"))
  (set `local.LocalSlotArray` (`|GetArrayItem` (`/Game/Blueprints/Interaction/AC_Inventory.Contents` `Source Inventory`) `Source Index`))
  (if (< `Destination Index` 0)
    (if (not (== (`.ItemID_2_84EE75DA4BEB4296A41792A283778ECC` (break `/Game/Blueprints/Interaction/STR_InventorySlots` (`local.LocalSlotArray`))) (`.ItemID_2_84EE75DA4BEB4296A41792A283778ECC` (break `/Game/Blueprints/Interaction/STR_InventorySlots` (`|GetArrayItem` (`self.Contents`) (`local.Destination Index`))))))
      (`KismetArrayLibrary.Array_Set` (`/Game/Blueprints/Interaction/AC_Inventory.Contents` (`local.Source Inventory`)) (`local.Source Index`) (`|GetArrayItem` (`self.Contents`) (`local.Destination Index`)))
      (`KismetArrayLibrary.Array_Set` (`self.Contents`) (`local.Destination Index`) (`local.LocalSlotArray`))
      (`self.MC_Update`)
      (`self.MC_Update` (`local.Source Inventory`)))))