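; Actor component that gives the player character a toggleable flashlight.
; The IA_Flashlight Enhanced Input action checks the FlashlightActive flag on Started and calls the matching on or off function.
; Each function casts the owner to SP_PlayerCharacter, shows or hides its SpotLight and updates the flag.
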(event `EnhancedInput|/Game/Player/Input/IA_Flashlight`
  (params (ActionValue :type Boolean) (ElapsedSeconds :type "Float (double-precision)") (TriggeredSeconds :type "Float (double-precision)") (InputAction :type "InputAction Object Reference" :default "/Game/Player/Input/IA_Flashlight.IA_Flashlight"))
  (:`Started`
    (if (`self.FlashlightActive`)
      (`self.fnFlashlightOff`)
      (else
        (`self.fnFlashlightOn`)))))

(fn `fnFlashlightOff`
  (`SceneComponent.SetVisibility` (`/Game/Player/SP_PlayerCharacter.SpotLight` (cast `/Game/Player/SP_PlayerCharacter` (`self.GetOwner`) :!pure true)) false false)
  (set `self.FlashlightActive` false))

(fn `fnFlashlightOn`
  (`SceneComponent.SetVisibility` (`/Game/Player/SP_PlayerCharacter.SpotLight` (cast `/Game/Player/SP_PlayerCharacter` (`self.GetOwner`) :!pure true)) true false)
  (set `self.FlashlightActive` true))