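; Inventory actor component that stores item ID and count pairs in a struct array and looks up quest item data in DT_QuestItems.
; Add appends an entry; Use removes through a query that needs an exact count match but returns after checking only the first slot.
; Remove blanks the slot without shrinking the array.
; Loading, inspect and quest check are stubs, and the update dispatcher fires only through evUpdateInv.
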(event `evDebug`
  (`|ExecutionSequence`
    (:`then_0`
      (`KismetSystemLibrary.PrintString` "Debug = on")
      (`KismetSystemLibrary.PrintString` (`KismetStringLibrary.Conv_IntToString` (`KismetArrayLibrary.Array_Length` (`self.STR_InventoryItem`)))))
    (:`then_1`
      (for _array_element (`self.STR_InventoryItem`)
        (bind (_id _count) (break `/Game/Data/Structs/STR_InventoryItem` _array_element))
        (`KismetSystemLibrary.PrintString` (`KismetStringLibrary.Concat_StrStr` "Have " (`KismetStringLibrary.Conv_IntToString` _count) " " _id))))))

(event `self.ReceiveBeginPlay`
  (bind (_success _loaded_inv_size) (`self.fnLoadInv`))
  (`KismetArrayLibrary.Array_Resize` (`self.STR_InventoryItem`) _loaded_inv_size))

(event `evUpdateInv`
  (`self.dpInvUpdated`))

(fn `fnAdd`
  (params (ItemID :type Name) (Quantity :type Integer))
  (returns (Success :type Boolean))
  (bind _result (`/Engine/EditorBlueprintResources/StandardMacros.IncrementInt` (`KismetArrayLibrary.Array_Length` (`self.STR_InventoryItem`)))
    (:`  `
      (`KismetArrayLibrary.Array_Resize` (`self.STR_InventoryItem`) _result)
      (`KismetArrayLibrary.Array_Set` (`self.STR_InventoryItem`) (- (`KismetArrayLibrary.Array_Length` (`self.STR_InventoryItem`)) 1) (make `/Game/Data/Structs/STR_InventoryItem` (`KismetStringLibrary.Conv_NameToString` ItemID) Quantity))
      (`KismetSystemLibrary.PrintString` (`KismetStringLibrary.Concat_StrStr` "Added" (`KismetStringLibrary.Conv_NameToString` (`local.ItemID`)) "to Inventory."))
      (return true))))

(fn `fnCheckQuest`
  (params (ItemID :type Name) (Quantity :type Integer)))

(fn `fnGetItemData`
  (params (ItemID :type Name))
  (returns (`Out Row` :type "/Game/Blueprints/Structs/STR_QuestItems Structure"))
  (bind _returnvalue (`|GetDataTableRow` "/Game/Blueprints/Miscellaneous/DT_QuestItems.DT_QuestItems" ItemID)
    (:`then`
      (return _returnvalue))))

(fn `fnInspect`
  (params (Index :type Integer)))

(fn `fnLoadInv`
  (returns (Success :type Boolean) (`Loaded Inv Size` :type Integer))
  (return true (`KismetArrayLibrary.Array_Length` (`self.STR_InventoryItem`))))

(fn `fnQueuryItem`
  (params (ItemID :type Name) (Quantity :type Integer))
  (returns (`Item found` :type Boolean) (SlotIndex :type Integer))
  (for (_array_element _array_index) (`self.STR_InventoryItem`)
    (bind (_id _count) (break `/Game/Data/Structs/STR_InventoryItem` _array_element))
    (if (and (== ItemID _id) (== _count Quantity))
      (return true _array_index)
      (else
        (`KismetSystemLibrary.PrintString` "Don't have the item")
        (return false -1)))))

(fn `fnRemove`
  (params (SlotIndex :type Integer))
  (`KismetArrayLibrary.Array_Set` (`self.STR_InventoryItem`) SlotIndex (make `/Game/Data/Structs/STR_InventoryItem` "")))

(fn `fnUse`
  (params (ItemID :type Name) (Quantity :type Integer))
  (returns (Success :type Boolean))
  (bind (_item_found _slotindex) (`self.fnQueuryItem` ItemID Quantity))
  (if _item_found
    (`self.fnRemove` _slotindex)
    (return true)
    (else
      (return false))))