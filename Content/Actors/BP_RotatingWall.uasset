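; BP_RotatingWall is a wall actor that periodically turns 90 degrees around its yaw axis.
; A looping timer set on BeginPlay fires every Cooldowntime and, unless a turn is already running, captures the current rotation and a target 90 degrees further.
; A timeline lerps the actor between them and clears the IsRotating guard when finished.
; The construction script places the actor from its Location and Rotation variables.
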(event `self.ReceiveBeginPlay`
  (`KismetSystemLibrary.K2_SetTimer` null "evStartRotate" (`self.Cooldowntime`) true))

(event `evStartRotate`
  (if (not (`self.bIsRotating`))
    (set `self.bIsRotating` true)
    (bind _output_get (set `self.StartRotation` (`self.K2_GetActorRotation`)))
    (set `self.EndRotation` (`KismetMathLibrary.MakeRotator` (.roll _output_get) (.pitch _output_get) (+ (.yaw _output_get) 90.0)))
    (bind (_direction _alpha) (`Timeline|TL_WallRotation` :!via `PlayFromStart`)
      (:`Update`
        (`self.K2_SetActorRotation` (`KismetMathLibrary.RLerp` (`self.StartRotation`) (`self.EndRotation`) _alpha)))
      (:`Finished`
        (set `self.bIsRotating` false)))))

(fn `UserConstructionScript`
  (`self.K2_SetActorLocationAndRotation` (`self.Location`) (`self.Rotation`)))