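; Master dialogue actor: a world object, interactable but neither examinable nor pickable, that starts a conversation when used.
; Interact creates W_Dialogue, starts CurrentDialogueAsset on DialogueComponent and switches to UI-only input with a cursor.
; Turn on/off events toggle its trace response, two hint spheres and icons, whose visibility follows player overlap and a MainGoal flag.
; The construction script applies mesh, hidden-mesh collision, hint layout and debug visibility.
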(event `self.ReceiveBeginPlay`
  ;[1 1 1] Begin Play
  (if (`self.InitiallyActive?`)
    (`self.fnToggleOnInteraction`)
    (else
      (`self.fnToggleOffInteraction`))))

(event `/Game/Blueprints/BPInterfaces/BPI_FlowControl.Turn On`
  ;[1 1 1] Turn On
  (`self.fnToggleOnInteraction`))

(event `/Game/Blueprints/BPInterfaces/BPI_FlowControl.Turn Off`
  ;[1 1 1] Turn Off
  (`self.fnToggleOffInteraction`))

(event `/Game/Blueprints/BPInterfaces/BPi_Interact.ShowHUD`
  ; Hint Logic
  (if (`PrimitiveComponent.IsOverlappingActor` (`self.innerSphereCollision`) (`GameplayStatics.GetPlayerCharacter` 0))
    (`SceneComponent.SetVisibility` (`self.innerInteractionIcon`) true false)
    (if (`self.MainGoal?`)
      (`SceneComponent.SetVisibility` (`self.outerInteractionIcon`) false false))
    (else
      (`SceneComponent.SetVisibility` (`self.innerInteractionIcon`) false false :!label _label)
      (if (`self.MainGoal?`)
        (`SceneComponent.SetVisibility` (`self.outerInteractionIcon`) true false)))))

(event `/Game/Blueprints/BPInterfaces/BPi_Interact.HideHUD`
  ; Hint Logic
  (if (`PrimitiveComponent.IsOverlappingActor` (`self.innerSphereCollision`) (`GameplayStatics.GetPlayerCharacter` 0))
    (goto _label)))

(event `self.outerSphereCollision.OnComponentBeginOverlap`
  (params (OverlappedComponent :type "PrimitiveComponent Object Reference") (OtherActor :type "Actor Object Reference") (OtherComp :type "PrimitiveComponent Object Reference") (OtherBodyIndex :type Integer) (bFromSweep :type Boolean) (SweepResult :type "HitResult Structure (by ref)"))
  ; Hint Sphere Overlap
  (if (and (== OtherActor (`GameplayStatics.GetPlayerCharacter` 0)) (`self.MainGoal?`))
    (`SceneComponent.SetVisibility` (`self.innerInteractionIcon`) true false)))

(event `self.outerSphereCollision.OnComponentEndOverlap`
  (params (OverlappedComponent :type "PrimitiveComponent Object Reference") (OtherActor :type "Actor Object Reference") (OtherComp :type "PrimitiveComponent Object Reference") (OtherBodyIndex :type Integer))
  ; Hint Sphere Overlap
  (if (and (`self.MainGoal?`) (== (`GameplayStatics.GetPlayerCharacter` 0) OtherActor))
    (`SceneComponent.SetVisibility` (`self.outerInteractionIcon`) false false)))

(event `/Game/Blueprints/BPInterfaces/BPI_FlowControl.Main Goal On`
  ; Main Quest Seetup
  (set `self.MainGoal?` true))

(event `/Game/Blueprints/BPInterfaces/BPI_FlowControl.Main Goal Off`
  ; Main Quest Seetup
  (set `self.MainGoal?` false))

(event `/Game/Blueprints/BPInterfaces/BPi_Interact.Interact`
  (params (PlayerCharacter :type "/Game/Player/SP_PlayerCharacter Object Reference"))
  (bind _returnvalue (`GameplayStatics.GetPlayerController` 0))
  ; Interaction
  (`|ExecutionSequence`
    (:`then_0`
      (bind _returnvalue_2 (`|CreateWidget` "/Game/UI/Dialogues/W_Dialogue.W_Dialogue_C" _returnvalue (`self.DialogueComponent`)))
      (`UserWidget.AddToViewport` _returnvalue_2 0)
      (`KismetSystemLibrary.PrintString` "Dialog started")
      (`/Game/Data/Dialogues/DialogueComponent.fnStartDialogue` (`self.DialogueComponent`) (`self.CurrentDialogueAsset`)))
    (:`then_1`
      (`WidgetBlueprintLibrary.SetInputMode_UIOnlyEx` _returnvalue _returnvalue_2)
      (set `PlayerController.bShowMouseCursor` true _returnvalue))))

(fn `fnToggleOffInteraction`
  (`PrimitiveComponent.SetCollisionResponseToChannel` (`self.StaticMesh`) "ECC_GameTraceChannel1" "ECR_Ignore")
  (`PrimitiveComponent.SetCollisionEnabled` (`self.innerSphereCollision`) "NoCollision")
  (`PrimitiveComponent.SetCollisionEnabled` (`self.outerSphereCollision`) "NoCollision")
  (`SceneComponent.SetHiddenInGame` (`self.innerInteractionIcon`) true false)
  (`SceneComponent.SetHiddenInGame` (`self.outerInteractionIcon`) true false))

(fn `fnToggleOnInteraction`
  (`PrimitiveComponent.SetCollisionResponseToChannel` (`self.StaticMesh`) "ECC_GameTraceChannel1" "ECR_Block")
  (`PrimitiveComponent.SetCollisionEnabled` (`self.outerSphereCollision`) "QueryOnly")
  (`PrimitiveComponent.SetCollisionEnabled` (`self.innerSphereCollision`) "QueryOnly")
  (`SceneComponent.SetHiddenInGame` (`self.innerInteractionIcon`) false false)
  (`SceneComponent.SetHiddenInGame` (`self.outerInteractionIcon`) false false))

(fn `IsExaminable`
  (returns (IsExaminable :type Boolean))
  (return false))

(fn `IsInteractable`
  (returns (IsInteractable :type Boolean))
  (return true))

(fn `IsPickable`
  (returns (IsPickable :type Boolean))
  (return false))

(fn `UserConstructionScript`
  (bind _staticmesh (`self.StaticMesh`))
  (`|ExecutionSequence`
    (:`then_0`
      ; Mesh Setup
      (`StaticMeshComponent.SetStaticMesh` _staticmesh (`self.ItemMesh`))
      (if (`self.MeshHidden?`)
        (`SceneComponent.SetVisibility` _staticmesh false false)
        (`PrimitiveComponent.SetCollisionResponseToAllChannels` _staticmesh "ECR_Ignore")
        (`PrimitiveComponent.SetCollisionResponseToChannel` _staticmesh "ECC_GameTraceChannel1" "ECR_Block")
        (else
          (`SceneComponent.SetVisibility` _staticmesh true false)
          (`PrimitiveComponent.SetCollisionResponseToAllChannels` _staticmesh "ECR_Block"))))
    (:`then_1`
      ; Hint Position
      (`SphereComponent.SetSphereRadius` (`self.outerSphereCollision`) (`self.HintSphereRadius`) true)
      (`SphereComponent.SetSphereRadius` (`self.innerSphereCollision`) (`self.InterSphereRadius`) true)
      (`SceneComponent.K2_SetRelativeLocation` (`self.innerInteractionIcon`) (`self.HintLocation`) false false)
      (`SceneComponent.K2_SetRelativeLocation` (`self.outerInteractionIcon`) (`self.HintLocation`) false false))
    (:`then_2`
      ;[1 1 1] Debuggin Mode
      (if (`self.DebugMode`)
        (`SceneComponent.SetVisibility` (`self.outerSphereCollision`) true false)
        (`SceneComponent.SetVisibility` (`self.innerSphereCollision`) true false)
        (`SceneComponent.SetVisibility` (`self.innerInteractionIcon`) true false)
        (`SceneComponent.SetVisibility` (`self.outerInteractionIcon`) true false)
        (else
          (`SceneComponent.SetVisibility` (`self.outerSphereCollision`) false false)
          (`SceneComponent.SetVisibility` (`self.innerSphereCollision`) false false)
          (`SceneComponent.SetVisibility` (`self.innerInteractionIcon`) false false)
          (`SceneComponent.SetVisibility` (`self.outerInteractionIcon`) false false))))))